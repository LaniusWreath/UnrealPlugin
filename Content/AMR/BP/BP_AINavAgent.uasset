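; AI-navigated character simulating an autonomous mobile robot (AMR) that travels between placer stations for welding, painting, storage and charging.
; It uses AIMoveTo, parks by timeline rotation, then works for the placer's set time.
; A state machine fires event dispatchers, sets velocity and changes the cargo's look by placer tag.
; A looping timer refreshes its 3D status widget and HTTP-posts telemetry, while WebSocket and data-container managers handle incoming data.
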(event `InitAMRAgentRoutine`
  ;[1 1 1] Inititalize
  (`self.Initialize AMR DataManagers`)
  (`self.InitAMRDataContainerDatas`)
  (`self.SetAMRState` "NewEnumerator0"))

(event `Initialize AMR DataManagers`
  (`|ExecutionSequence`
    (:`then_0`
      ;[0.1686 0.06667 0.06274] Initialize HTTP
      (bind _returnvalue (`SFCHttpManager.CreateHttpManagerInstance` self "/Script/SmartFactory.SFCHttpManager"))
      (bind _output_get (set `self.HTTPManagerRef` _returnvalue)))
    (:`then_1`
      ;[0.1119 0.1384 0.2502] Initialize WebSocket
      (bind _returnvalue_2 (`SFCDataManageUtilities.CreateEmptyDataContainer` self))
      (set `self.AMRDataContainerRef` _returnvalue_2)
      (bind _returnvalue_3 (`SFCWebSocketManager.CreateWebSocketManagerInstance` self "/Script/SmartFactory.SFCWebSocketManager"))
      (bind _output_get_2 (set `self.WebSocketManagerRef` _returnvalue_3))
      (add `SFCWebSocketManager.OnMessageReceivedEvent` _output_get_2 (`|CreateDelegate` :!event `UpdateDataContainer`))
      (`self.InitAMRDataContainerDatas`))
    (:`then_2`
      ;[0.6829 1 0.6305] Initialize 3DWidget
      (`KismetSystemLibrary.Delay` 0.2)
      (bind _aswbp_sfc_amr_3d (cast `/SmartFactory/Widget/MemberWidgets/WBP_SFC_AMR_3D` (`WidgetComponent.GetUserWidgetObject` (`self.Widget`))))
      (set `self.WBP_AMR3D` _aswbp_sfc_amr_3d)
      (`self.Init3DWidgetData`)
      (`KismetSystemLibrary.K2_SetTimer` null "TimerRoutine" (`self.CurrentUnitTime`) true true))))

(event `MoveAMRtoAMRPlacer`
  (params (InAMRPlacerRef :type "/SmartFactory/Blueprint/BP_AMRPlacer Object Reference"))
  (bind (_returnvalue_roll _returnvalue_pitch _returnvalue_yaw) (`KismetMathLibrary.BreakRotator` (`self.K2_GetActorRotation`)))
  ;[1 1 1] Animation
  (bind _output_get (set `self.CurPlacer` InAMRPlacerRef))
  (set `self.CurAMRDestination` (`KismetSystemLibrary.GetDisplayName` _output_get))
  (`|AIMoveTo` self (`SceneComponent.K2_GetComponentLocation` (`/SmartFactory/Blueprint/BP_AMRPlacer.PlacerPivot` _output_get)) null 0.1
    (:`OnSuccess`
      ;;[1 1 1] Parking
      (set `self.CurrentRotation` _returnvalue_yaw)
      (bind _output_get_2 (set `self.DeltaYaw` (- (`self.TargetRotation`) (`self.CurrentRotation`))))
      (if (> _output_get_2 0.0)
        (set `self.TargetRotation` 90.0)
        (bind (_direction `_새_트랙_0`) (`Timeline|타임라인` :!via `PlayFromStart` :!label _label)
          (:`Update`
            (`self.K2_SetActorRelativeRotation` (`KismetMathLibrary.MakeRotator` 0.0 0.0 (`KismetMathLibrary.Lerp` (`self.CurrentRotation`) (`self.TargetRotation`) `_새_트랙_0`))))
          (:`Finished`
            (`self.SetAMRState` "NewEnumerator5")
            (`self.SetAMRState` "NewEnumerator3")
            (`self.AMRStartWorking` (`/SmartFactory/Blueprint/BP_AMRPlacer.WorkTime` (`self.CurPlacer`)))))
        (else
          (set `self.TargetRotation` 270.0)
          (goto _label :!via `PlayFromStart`))))))

(event `self.ReceiveDestroyed`
  ;[0.1119 0.1384 0.2502] Disconnect WebSocket
  (`/Engine/EditorBlueprintResources/StandardMacros.IsValid` (`self.WebSocketManagerRef`) :!label _label_2
    (:`Is Valid`
      (`SFCWebSocketManager.Disconnect` (`self.WebSocketManagerRef`)))))

(event `self.ReceiveEndPlay`
  (params (EndPlayReason :type "EEndPlayReason Enum" :default "Destroyed"))
  ;[0.1119 0.1384 0.2502] Disconnect WebSocket
  (goto _label_2))

(event `Key|T`
  (params (Key :type "Key Structure"))
  (bind _returnvalue (`GameplayStatics.GetPlayerController` 0))
  ;[1 1 1] Input
  (:`Pressed`
    (`/Engine/EditorBlueprintResources/StandardMacros.FlipFlop`
      (:`A`
        (set `PlayerController.bShowMouseCursor` false _returnvalue)
        (`Controller.SetIgnoreMoveInput` _returnvalue false)
        (`Controller.SetIgnoreLookInput` _returnvalue false))
      (:`B`
        (set `PlayerController.bShowMouseCursor` true _returnvalue)
        (`Controller.SetIgnoreMoveInput` _returnvalue true)
        (`Controller.SetIgnoreLookInput` _returnvalue true)))))

(event `self.Box.OnComponentBeginOverlap`
  (params (OverlappedComponent :type "PrimitiveComponent Object Reference") (OtherActor :type "Actor Object Reference") (OtherComp :type "PrimitiveComponent Object Reference") (OtherBodyIndex :type Integer) (bFromSweep :type Boolean) (SweepResult :type "HitResult Structure (by ref)"))
  (set `self.CurCollisionDetected` (`|EnumEquality` (`self.CurAMRState`) "NewEnumerator2")))

(event `CallPostData`
  (`self.PostAMRDataToServer`))

(event `self.Box.OnComponentEndOverlap`
  (params (OverlappedComponent :type "PrimitiveComponent Object Reference") (OtherActor :type "Actor Object Reference") (OtherComp :type "PrimitiveComponent Object Reference") (OtherBodyIndex :type Integer))
  (if (`self.CurCollisionDetected`)
    (set `self.CurCollisionDetected` false)))

(fn `AMRStartWorking`
  (params (Time :type "Float (single-precision)"))
  (`KismetSystemLibrary.K2_SetTimer` null "SendMessageAMRWorkingDone" Time))

(fn `ConnectSocket`
  (bind _websocketmanagerref (`self.WebSocketManagerRef`))
  (`/Engine/EditorBlueprintResources/StandardMacros.IsValid` _websocketmanagerref
    (:`Is Valid`
      (`SFCWebSocketManager.Connect` _websocketmanagerref (`self.WebSocketAddress`)))))

(fn `EditorFunction_InitAMRDatas`
  (params (HTTPURL :type String) (WebSocketAddress :type String) (InAMRAddress :type Integer) (InVelocity :type "Float (double-precision)") (InSFCManagerRef :type "/SmartFactory/Blueprint/Logics/BP_SFCManager Object Reference"))
  (set `self.HTTPURL` HTTPURL)
  (set `self.WebSocketAddress` WebSocketAddress)
  (set `self.AMRID` InAMRAddress)
  (set `self.CurVelocity` InVelocity)
  (set `self.SFCManagerRef` InSFCManagerRef))

(fn `EnrollAMRPlacerActors`
  (params (TargetAMRPlacer :type "Array of /SmartFactory/Blueprint/BP_AMRPlacer Object Reference"))
  (set `self.TargetAMRPlacer` TargetAMRPlacer))

(fn `GetAMRData`
  (returns (OutAMRData :type "GenericData Structure (by ref)"))
  (return (`SFCDataContainer.GetData` (`self.AMRDataContainerRef`))))

(fn `Init3DWidgetData`
  (bind (_returnvalue_x _returnvalue_y _returnvalue_z) (`KismetMathLibrary.BreakVector` (`self.K2_GetActorLocation`)))
  (bind (_returnvalue_roll _returnvalue_pitch _returnvalue_yaw) (`KismetMathLibrary.BreakRotator` (`self.K2_GetActorRotation`)))
  (message `/SmartFactory/Blueprint/Logics/BPIF_InitRobotState.InitAMRStateText` (`self.WBP_AMR3D`) "" (`KismetTextLibrary.Conv_StringToText` (`KismetSystemLibrary.GetDisplayName` self)) (`KismetTextLibrary.Conv_StringToText` (`|GetEnumeratorNameAsString` (`self.CurAMRState`))) (`KismetTextLibrary.Conv_StringToText` (`self.CurAMRDestination`)) (`KismetTextLibrary.Conv_DoubleToText` _returnvalue_x "HalfToEven") (`KismetTextLibrary.Conv_DoubleToText` _returnvalue_y "HalfToEven") (`KismetTextLibrary.Conv_DoubleToText` _returnvalue_z "HalfToEven") (`KismetTextLibrary.Conv_IntToText` (`self.CurHeight`)) (`KismetTextLibrary.Conv_DoubleToText` _returnvalue_yaw "HalfToEven") (`KismetTextLibrary.Conv_DoubleToText` (/ (`self.CurVelocity`) 100.0) "HalfToEven") "" (`KismetTextLibrary.Conv_BoolToText` (`self.CurCollisionDetected`))))

(fn `InitAMRDataContainerDatas`
  (locals (NewLocalVar :type Integer))
  (bind (_returnvalue_x _returnvalue_y _returnvalue_z) (`KismetMathLibrary.BreakVector` (`self.K2_GetActorLocation`)))
  (bind (_returnvalue_roll _returnvalue_pitch _returnvalue_yaw) (`KismetMathLibrary.BreakRotator` (`self.K2_GetActorRotation`)))
  (`SFCDataContainer.SetData` (`self.AMRDataContainerRef`) (make `GenericData` (`KismetSystemLibrary.GetDisplayName` self) "" (`/SmartFactory/Blueprint/Logics/BPFL_AMRDataParsing.MakeAMRDataMap_String` (`KismetStringLibrary.Conv_IntToString` (`self.AMRID`)) (`|GetEnumeratorNameAsString` (`self.CurAMRState`)) (`self.CurAMRDestination`) (`KismetStringLibrary.Conv_DoubleToString` _returnvalue_x) (`KismetStringLibrary.Conv_DoubleToString` _returnvalue_y) (`KismetStringLibrary.Conv_DoubleToString` _returnvalue_z) (`KismetStringLibrary.Conv_IntToString` (`self.CurHeight`)) (`KismetStringLibrary.Conv_DoubleToString` _returnvalue_yaw) (`KismetStringLibrary.Conv_DoubleToString` (`self.CurVelocity`)) (`KismetStringLibrary.Conv_IntToString` (`self.CurBattery`)) (`KismetStringLibrary.Conv_BoolToString` (`self.CurCollisionDetected`))))))

(fn `PostAMRDataToServer`
  (bind (_returnvalue_roll _returnvalue_pitch _returnvalue_yaw) (`KismetMathLibrary.BreakRotator` (`self.K2_GetActorRotation`)))
  (bind (_returnvalue_x _returnvalue_y _returnvalue_z) (`KismetMathLibrary.BreakVector` (`self.K2_GetActorLocation`)))
  (`SFCHttpManager.MakePostRequest` (`self.HTTPManagerRef`) (`self.HTTPURL`) (`|MakeMap` "accept" "application/json" "Content-Type" "application/json") (`/SmartFactory/Blueprint/Logics/BPFL_AMRDataParsing.MakeAMRDataMap_String` (`KismetSystemLibrary.GetDisplayName` self) (`|GetEnumeratorNameAsString` (`self.CurAMRState`)) (`self.CurAMRDestination`) (`KismetStringLibrary.Conv_DoubleToString` _returnvalue_x) (`KismetStringLibrary.Conv_DoubleToString` _returnvalue_y) (`KismetStringLibrary.Conv_DoubleToString` _returnvalue_z) (`KismetStringLibrary.Conv_IntToString` (`self.CurHeight`)) (`KismetStringLibrary.Conv_DoubleToString` _returnvalue_yaw) (`KismetStringLibrary.Conv_DoubleToString` (/ (`self.CurVelocity`) 100.0)) (`KismetStringLibrary.Conv_IntToString` (`self.CurBattery`)) (`KismetStringLibrary.Conv_BoolToString` (`self.CurCollisionDetected`)))))

(fn `PrintHTTPResponse`
  (bind _httpmanagerref (`self.HTTPManagerRef`))
  (`KismetSystemLibrary.PrintString` (`SFCHttpManager.GetTempResultResponseString` _httpmanagerref))
  (`KismetSystemLibrary.PrintString` (`SFCHttpManager.GetResultResponseString` _httpmanagerref)))

(fn `SendMessageAMRWorkingDone`
  (`self.ED_AMRWorkingDone` self (`self.CurPlacer`))
  (`self.SetAMRState` "NewEnumerator2"))

(fn `SetAMRState`
  (params (InState :type "/SmartFactory/AMR/BP/ENUM_AMRState Enum" :default "NewEnumerator0"))
  (bind _output_get (set `self.CurAMRState` InState))
  (switch `/SmartFactory/AMR/BP/ENUM_AMRState` _output_get
    (:`NewEnumerator0`
      (`self.ED_AMRInitializing` self)
      (set `self.CurVelocity` 0.0))
    (:`NewEnumerator1`
      (`self.ED_AMRStartWaiting` self)
      (set `self.CurVelocity` 0.0))
    (:`NewEnumerator2`
      (`self.ED_AMRStartMoving` self)
      (set `self.CurVelocity` (`CharacterMovementComponent.MaxWalkSpeed` (`self.CharacterMovement`))))
    (:`NewEnumerator5`
      (`self.ED_AMRArrivied` (`self.CurPlacer`)))
    (:`NewEnumerator3`
      (`self.ED_AMRWorking` self (`self.CurPlacer`))
      (set `self.CurCollisionDetected` false)
      (switch `name` (`|GetArrayItem` (`Actor.Tags` (`self.CurPlacer`)))
        (:`Welding`
          (set `self.CurWorkState` "NewEnumerator0")
          (`SceneComponent.SetVisibility` (`self.Bagage`) true false))
        (:`Painting`
          (set `self.CurWorkState` "NewEnumerator1")
          (`PrimitiveComponent.SetMaterial` (`self.Bagage`) 0 "/SmartFactory/Material/M_SolidWhite.M_SolidWhite"))
        (:`Storaging`
          (set `self.CurWorkState` "NewEnumerator2")
          (`SceneComponent.SetVisibility` (`self.Bagage`) false false))
        (:`Charging`
          (set `self.CurWorkState` "NewEnumerator3")
          (`PrimitiveComponent.SetMaterial` (`self.Bagage`) 0 "/Engine/EngineMaterials/DefaultMaterial.DefaultMaterial"))))
    (:`NewEnumerator8`
      (`self.ED_AMRWorkingDone` self (`self.CurPlacer`)))))

(fn `TimerRoutine`
  (`self.Update 3DWidget Data`)
  (`self.PostAMRDataToServer`))

(fn `Update 3DWidget Data`
  (bind (_returnvalue_x _returnvalue_y _returnvalue_z) (`KismetMathLibrary.BreakVector` (`self.K2_GetActorLocation`)))
  (bind (_returnvalue_roll _returnvalue_pitch _returnvalue_yaw) (`KismetMathLibrary.BreakRotator` (`self.K2_GetActorRotation`)))
  (`/SmartFactory/Widget/MemberWidgets/WBP_SFC_AMR_3D.InitAMRStateText` (`self.WBP_AMR3D`) (`KismetTextLibrary.Conv_StringToText` (`KismetSystemLibrary.GetDisplayName` self)) (`KismetTextLibrary.Conv_StringToText` (`KismetSystemLibrary.GetDisplayName` self)) (`KismetTextLibrary.Conv_StringToText` (`|GetEnumeratorNameAsString` (`self.CurAMRState`))) (`KismetTextLibrary.Conv_StringToText` (`self.CurAMRDestination`)) (`KismetTextLibrary.Conv_DoubleToText` _returnvalue_x "HalfToEven") (`KismetTextLibrary.Conv_DoubleToText` _returnvalue_y "HalfToEven") (`KismetTextLibrary.Conv_DoubleToText` _returnvalue_z "HalfToEven") (`KismetTextLibrary.Conv_IntToText` (`self.CurHeight`)) (`KismetTextLibrary.Conv_DoubleToText` _returnvalue_yaw "HalfToEven") (`KismetTextLibrary.Conv_DoubleToText` (/ (`self.CurVelocity`) 100.0) "HalfToEven") "" (`KismetTextLibrary.Conv_BoolToText` (`self.CurCollisionDetected`))))

(fn `UpdateDataContainer`
  (params (ReceivedMessage :type String))
  (bind _returnvalue (`SFCDataManageUtilities.ParseJsonStringToMap` ReceivedMessage))
  (bind _returnvalue_2 (`SFCDataManageUtilities.ParseJsonStringToMap` (`BlueprintMapLibrary.Map_Find` _returnvalue "data")))
  (`SFCDataManageUtilities.UpdateDataContainer` (`self.AMRDataContainerRef`) (make `GenericData` "" "" (`/SmartFactory/Blueprint/Logics/BPFL_AMRDataParsing.MakeAMRDataMap_String` (`BlueprintMapLibrary.Map_Find` _returnvalue_2 "amrType") (`BlueprintMapLibrary.Map_Find` _returnvalue_2 "state") (`BlueprintMapLibrary.Map_Find` _returnvalue_2 "destination") (`BlueprintMapLibrary.Map_Find` _returnvalue_2 "locationX") (`BlueprintMapLibrary.Map_Find` _returnvalue_2 "locationY") (`BlueprintMapLibrary.Map_Find` _returnvalue_2 "locationZ") (`BlueprintMapLibrary.Map_Find` _returnvalue_2 "height") (`BlueprintMapLibrary.Map_Find` _returnvalue_2 "direction") (`BlueprintMapLibrary.Map_Find` _returnvalue_2 "velocity") (`BlueprintMapLibrary.Map_Find` _returnvalue_2 "battery") (`BlueprintMapLibrary.Map_Find` _returnvalue_2 "collisionEtected"))))
  (`self.ED_AMRSocketDataSaved` (`KismetSystemLibrary.GetDisplayName` self)))

(fn `UserConstructionScript`
  (bind (_returnvalue_x _returnvalue_y _returnvalue_z) (`KismetMathLibrary.BreakVector` (`self.K2_GetActorLocation`)))
  (bind (_returnvalue_roll _returnvalue_pitch _returnvalue_yaw) (`KismetMathLibrary.BreakRotator` (`self.K2_GetActorRotation`)))
  (`/SmartFactory/Widget/MemberWidgets/WBP_SFC_AMR_3D.InitAMRStateText` (`self.WBP_AMR3D`) "" (`KismetTextLibrary.Conv_StringToText` (`KismetSystemLibrary.GetDisplayName` self)) (`KismetTextLibrary.Conv_StringToText` (`|GetEnumeratorNameAsString` (`self.CurAMRState`))) (`KismetTextLibrary.Conv_StringToText` (`self.CurAMRDestination`)) (`KismetTextLibrary.Conv_DoubleToText` _returnvalue_x "HalfToEven") (`KismetTextLibrary.Conv_DoubleToText` _returnvalue_y "HalfToEven") (`KismetTextLibrary.Conv_DoubleToText` _returnvalue_z "HalfToEven") (`KismetTextLibrary.Conv_IntToText` (`self.CurHeight`)) (`KismetTextLibrary.Conv_DoubleToText` _returnvalue_yaw "HalfToEven") (`KismetTextLibrary.Conv_DoubleToText` (`self.CurVelocity`) "HalfToEven") "" (`KismetTextLibrary.Conv_BoolToText` (`self.CurCollisionDetected`))))