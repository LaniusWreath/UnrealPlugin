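; BP_Cell_LYJ is a work cell that switches its robots and robot arms on and off as a BP_AINavAgent enters and leaves it.
; On CellBoundary begin overlap it starts work on each entry in Robots, playing MS_Spray at the world origin per robot, then operates each RobotArm entry.
; On end overlap it stops both sets, with no count of how many agents remain inside.
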(event `self.CellBoundary.OnComponentBeginOverlap`
  (params (OverlappedComponent :type "PrimitiveComponent Object Reference") (OtherActor :type "Actor Object Reference") (OtherComp :type "PrimitiveComponent Object Reference") (OtherBodyIndex :type Integer) (bFromSweep :type Boolean) (SweepResult :type "HitResult Structure (by ref)"))
  (cast `/SmartFactory/AMR/BP/BP_AINavAgent` OtherActor)
  (`|ExecutionSequence`
    (:`then_0`
      (for _array_element (`self.Robots`)
        (`GameplayStatics.PlaySoundAtLocation` "/SmartFactory/LYJ/Sound/MS_Spray.MS_Spray" (0.0 0.0 0.0) (struct) 1.0 1.0 0.0 null null null null)
        (`/SmartFactory/LYJ/BP/BP_IndustrialRobot.StartRobotWork` _array_element)))
    (:`then_1`
      (for _array_element_2 (`self.RobotArm`)
        (`/SmartFactory/Blueprint/BP_RobotArm.Operate` _array_element_2)))))

(event `self.CellBoundary.OnComponentEndOverlap`
  (params (OverlappedComponent :type "PrimitiveComponent Object Reference") (OtherActor :type "Actor Object Reference") (OtherComp :type "PrimitiveComponent Object Reference") (OtherBodyIndex :type Integer))
  (cast `/SmartFactory/AMR/BP/BP_AINavAgent` OtherActor)
  (`|ExecutionSequence`
    (:`then_0`
      (for _array_element (`self.Robots`)
        (`/SmartFactory/LYJ/BP/BP_IndustrialRobot.StopRobotWork` _array_element)))
    (:`then_1`
      (for _array_element_2 (`self.RobotArm`)
        (`/SmartFactory/Blueprint/BP_RobotArm.Stop` _array_element_2)))))

(fn `UserConstructionScript`
  (`parent.UserConstructionScript`))