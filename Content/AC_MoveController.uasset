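; Actor component that moves its owning BP_RackLoader from its start location to its move target.
; A looping 0.016 s timer, created paused and used instead of the owner's tick, advances Alpha by MoveSpeed and feeds lerped positions to MoveLoader.
; StartMovement unpauses it.
; On arrival it snaps to the target, waits one second, signals movement end, pauses the timer and resets Alpha.
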(event `self.ReceiveBeginPlay`
  (bind _asbp_rack_loader (cast `/SmartFactory/BP_RackLoader` (`self.GetOwner`)))
  (set `self.Owner` _asbp_rack_loader)
  ;[1 1 1] Owner에서의 event tick 대신
  (bind _returnvalue (`KismetSystemLibrary.K2_SetTimerDelegate` (delegate `Move`) 0.016 true))
  (bind _output_get (set `self.MoveTimer` _returnvalue))
  (`KismetSystemLibrary.K2_PauseTimerHandle` _output_get))

(event `Move`
  (bind _owner (`self.Owner`))
  (bind _owner_2 (`self.Owner`))
  (bind _output_get (set `self.Alpha` (`KismetMathLibrary.FMin` (+ (`self.Alpha`) (* (`self.MoveSpeed`) 0.016)) 1.0)))
  (if (>= _output_get 1.0)
    ;[1 1 1] 예외처리(혹시나 앞에서 완벽히 안 갔을 경우)
    (`/SmartFactory/BP_RackLoader.MoveLoader` _owner (`/SmartFactory/BP_RackLoader.MoveTargetLocation` _owner))
    (`KismetSystemLibrary.Delay` 1.0)
    (`self.EndMovement`)
    (`self.InitMovement`)
    (else
      (`/SmartFactory/BP_RackLoader.MoveLoader` (`self.Owner`) (`KismetMathLibrary.VLerp` (`/SmartFactory/BP_RackLoader.StartLocation` _owner_2) (`/SmartFactory/BP_RackLoader.MoveTargetLocation` _owner_2) (`self.Alpha`))))))

(event `StartMovement`
  (`KismetSystemLibrary.K2_UnPauseTimerHandle` (`self.MoveTimer`)))

(event `EndMovement`
  (`self.OnMovementEnd`)
  (`KismetSystemLibrary.K2_PauseTimerHandle` (`self.MoveTimer`)))

(event `InitMovement`
  (set `self.Alpha` 0.0))