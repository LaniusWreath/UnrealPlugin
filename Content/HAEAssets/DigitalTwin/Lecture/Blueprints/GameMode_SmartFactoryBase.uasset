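; GameMode for the Smart Factory digital twin that manages single-actor click selection and the robot arm UI.
; On BeginPlay it creates WBP_RobotArm, adds it to the viewport and exposes SetWidgetText to pass actor data into it.
; OnSelectableActorClicked tracks the current actor, toggling its selection message when re-clicked or moving it to the newly clicked actor.
; Deselecting by re-click also calls SetWidgetText with empty data.
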(event `SetWidgetText`
  (params (InActorData :type "/SmartFactory/HAEAssets/DigitalTwin/Lecture/Blueprints/STRT_ActorData Structure"))
  (`/SmartFactory/HAEAssets/DigitalTwin/Lecture/Widgets/WBP_RobotArm.SetTextFromActorData` (`self.WBP_RobotArmRef`) InActorData))

(event `self.ReceiveBeginPlay`
  (bind _returnvalue (`|CreateWidget` "/SmartFactory/HAEAssets/DigitalTwin/Lecture/Widgets/WBP_RobotArm.WBP_RobotArm_C"))
  (bind _output_get (set `self.WBP_RobotArmRef` _returnvalue))
  (`UserWidget.AddToViewport` (`self.WBP_RobotArmRef`) 0)
  (`UserWidget.AddToViewport` _output_get 0))

(event `OnSelectableActorClicked`
  (params (NewParam :type "Actor Object Reference"))
  (`/Engine/EditorBlueprintResources/StandardMacros.IsValid` (`self.CurrentSelectedActor`)
    (:`Is Valid`
      (if (== (`self.CurrentSelectedActor`) NewParam)
        (message `/SmartFactory/HAEAssets/DigitalTwin/Lecture/Blueprints/BPIF_SelectableActor.DisableSelection` (`self.CurrentSelectedActor`))
        (set `self.CurrentSelectedActor` null)
        (`self.SetWidgetText` (struct))
        (else
          (message `/SmartFactory/HAEAssets/DigitalTwin/Lecture/Blueprints/BPIF_SelectableActor.DisableSelection` (`self.CurrentSelectedActor`))
          (bind _output_get (set `self.CurrentSelectedActor` NewParam))
          (message `/SmartFactory/HAEAssets/DigitalTwin/Lecture/Blueprints/BPIF_SelectableActor.EnableSelection` _output_get))))
    (:`Is Not Valid`
      (bind _output_get_2 (set `self.CurrentSelectedActor` NewParam))
      (message `/SmartFactory/HAEAssets/DigitalTwin/Lecture/Blueprints/BPIF_SelectableActor.EnableSelection` _output_get_2))))

(fn `UserConstructionScript`)