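; Selectable smart-factory robot arm that cycles through a list of target locations while operating.
; A gated Tick moves the target at constant speed, yaws the stand toward it with an arcsine offset correction, and messages the mesh-relative position to the AnimInstance.
; Operate and Stop toggle that gate and the material-driven lights, and update ActorData.
; Clicks go to GameMode_SmartFactoryBase, whose widget shows the selected arm's data.
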(event `self.ReceiveTick`
  (params (DeltaSeconds :type "Float (single-precision)"))
  (`/Engine/EditorBlueprintResources/StandardMacros.Gate` true :!label _label
    (:`Exit`
      (set `self.TargetLocation` (+ (`self.TargetLocation`) (* (* (`KismetMathLibrary.Normal` (- (`|GetArrayItem` (`self.LocationList`) (`self.LocationIndex`)) (`self.TargetLocation`))) (`self.MovementSpeed`)) DeltaSeconds)))
      (if (< (`KismetMathLibrary.Vector_Distance` (`self.TargetLocation`) (`|GetArrayItem` (`self.LocationList`) (`self.LocationIndex`))) (* (`self.MovementSpeed`) DeltaSeconds))
        (set `self.TargetLocation` (`|GetArrayItem` (`self.LocationList`) (`self.LocationIndex`)))
        (set `self.LocationIndex` (mod (+ (`self.LocationIndex`) 1) (`KismetArrayLibrary.Array_Length` (`self.LocationList`)))))
      (`self.RefreshTargetLocation`))))

(event `OpenTickGate`
  (goto _label :!via `Open`))

(event `CloseTickGate`
  (goto _label :!via `Close`))

(event `RefreshTargetLocation`
  (`SceneComponent.K2_SetRelativeLocation` (`self.LocationReferenceScene`) (+ (`self.TargetLocation`) (0.0 0.0 75.0)) false false)
  (`SceneComponent.K2_SetRelativeRotation` (`self.RobotArmStand`) (`KismetMathLibrary.MakeRotator` 0.0 0.0 (- (.yaw (`KismetMathLibrary.FindLookAtRotation` (`SceneComponent.K2_GetComponentLocation` (`self.RobotArmStand`)) (`SceneComponent.K2_GetComponentLocation` (`self.LocationReferenceScene`)))) (`KismetMathLibrary.DegAsin` (/ 20.0 (`KismetMathLibrary.Vector_Distance` (`SceneComponent.K2_GetComponentLocation` (`self.LocationReferenceScene`)) (`SceneComponent.K2_GetComponentLocation` (`self.RobotArmStand`))))))) false false)
  (message `/SmartFactory/HAEAssets/DigitalTwin/Lecture/RobotArm/BPIF_AnimControl.SetVectorData` (`SkeletalMeshComponent.GetAnimInstance` (`self.SkeletalMesh`)) (.location (`KismetMathLibrary.MakeRelativeTransform` (`SceneComponent.K2_GetComponentToWorld` (`self.LocationReferenceScene`)) (`SceneComponent.K2_GetComponentToWorld` (`self.SkeletalMesh`)))) "TargetLocation"))

(event `self.ReceiveActorOnClicked`
  (params (ButtonPressed :type "Key Structure"))
  (`self.OnActorSelected`))

(event `SetNewOperationState`
  (params (InOperationState :type "/SmartFactory/HAEAssets/DigitalTwin/Lecture/Blueprints/Enum_OperationState Enum" :default "NewEnumerator0"))
  (bind _output_get (set `self.OperationState` InOperationState))
  (bind _structout (setmembers `/SmartFactory/HAEAssets/DigitalTwin/Lecture/Blueprints/STRT_ActorData` :`StructRef` (`self.ActorData`) :`OperationState` _output_get))
  (set `self.ActorData` _structout)
  (bind _asgame_mode_smart_factory_base (cast `/SmartFactory/HAEAssets/DigitalTwin/Lecture/Blueprints/GameMode_SmartFactoryBase` (`GameplayStatics.GetGameMode`)))
  (if (== (`/SmartFactory/HAEAssets/DigitalTwin/Lecture/Blueprints/GameMode_SmartFactoryBase.CurrentSelectedActor` _asgame_mode_smart_factory_base) self)
    (`/SmartFactory/HAEAssets/DigitalTwin/Lecture/Blueprints/GameMode_SmartFactoryBase.SetWidgetText` _asgame_mode_smart_factory_base (`self.ActorData`)))
  (switch `/SmartFactory/HAEAssets/DigitalTwin/Lecture/Blueprints/Enum_OperationState` (`self.OperationState`)
    (:`NewEnumerator0`
      (`|ExecutionSequence`
        (:`then_0`
          (`MeshComponent.SetScalarParameterValueOnMaterials` (`self.Cylinder`) "Intensity" 0.0)
          (`MeshComponent.SetScalarParameterValueOnMaterials` (`self.SphereLight1`) "Intensity" 0.0)
          (`MeshComponent.SetScalarParameterValueOnMaterials` (`self.SphereLight2`) "Intensity" 0.0)
          (`MeshComponent.SetScalarParameterValueOnMaterials` (`self.StateLightMesh`) "Intensity" 0.0)
          (set `self.LightState` 1)
          (`self.SetLightState`))
        (:`then_1`
          (`self.CloseTickGate`))))
    (:`NewEnumerator1`
      (`|ExecutionSequence`
        (:`then_0`
          (`MeshComponent.SetScalarParameterValueOnMaterials` (`self.Cylinder`) "Intensity" 100.0)
          (`MeshComponent.SetScalarParameterValueOnMaterials` (`self.SphereLight1`) "Intensity" 100.0)
          (`MeshComponent.SetScalarParameterValueOnMaterials` (`self.SphereLight2`) "Intensity" 100.0)
          (`MeshComponent.SetScalarParameterValueOnMaterials` (`self.StateLightMesh`) "Intensity" 100.0)
          (set `self.LightState` 3)
          (`self.SetLightState`))
        (:`then_1`
          (`self.OpenTickGate`))))))

(event `/SmartFactory/HAEAssets/DigitalTwin/Lecture/Blueprints/BPIF_SelectableActor.OnActorSelected`
  (bind _asgame_mode_smart_factory_base (cast `/SmartFactory/HAEAssets/DigitalTwin/Lecture/Blueprints/GameMode_SmartFactoryBase` (`GameplayStatics.GetGameMode`)))
  (`/SmartFactory/HAEAssets/DigitalTwin/Lecture/Blueprints/GameMode_SmartFactoryBase.OnSelectableActorClicked` _asgame_mode_smart_factory_base self))

(event `SetLightState`
  (bind _statelightmesh (`self.StateLightMesh`))
  (bind _lightstate (`self.LightState`))
  (`MeshComponent.SetScalarParameterValueOnMaterials` _statelightmesh "Light1On" (select `int` _lightstate :`0` 0.0 :`1` 1.0 :`2` 0.0 :`3` 0.0 :`4` 1.0 :!type "Float (single-precision)"))
  (`MeshComponent.SetScalarParameterValueOnMaterials` _statelightmesh "Light2On" (select `int` _lightstate :`0` 0.0 :`1` 0.0 :`2` 1.0 :`3` 0.0 :`4` 1.0 :!type "Float (single-precision)"))
  (`MeshComponent.SetScalarParameterValueOnMaterials` _statelightmesh "Light3On" (select `int` _lightstate :`0` 0.0 :`1` 0.0 :`2` 0.0 :`3` 1.0 :`4` 1.0 :!type "Float (single-precision)")))

(event `/SmartFactory/HAEAssets/DigitalTwin/Lecture/Blueprints/BPIF_SelectableActor.EnableSelection`
  (`SceneComponent.SetVisibility` (`self.SelectionPlane`) true false)
  (bind _asgame_mode_smart_factory_base (cast `/SmartFactory/HAEAssets/DigitalTwin/Lecture/Blueprints/GameMode_SmartFactoryBase` (`GameplayStatics.GetGameMode`)))
  (`/SmartFactory/HAEAssets/DigitalTwin/Lecture/Blueprints/GameMode_SmartFactoryBase.SetWidgetText` _asgame_mode_smart_factory_base (`self.ActorData`)))

(event `/SmartFactory/HAEAssets/DigitalTwin/Lecture/Blueprints/BPIF_SelectableActor.DisableSelection`
  (`SceneComponent.SetVisibility` (`self.SelectionPlane`) false false))

(event `Operate`
  (`self.SetNewOperationState` "NewEnumerator1"))

(event `Stop`
  (`self.SetNewOperationState` "NewEnumerator0"))

(fn `GetActorData`
  (returns (OutActorData :type "/SmartFactory/HAEAssets/DigitalTwin/Lecture/Blueprints/STRT_ActorData Structure"))
  (return (`self.ActorData`)))

(fn `UserConstructionScript`
  (bind _skeletalmesh (`self.SkeletalMesh`))
  (bind _statelightmesh (`self.StateLightMesh`))
  (bind _lightstate (`self.LightState`))
  (`self.RefreshTargetLocation`)
  (`MeshComponent.SetScalarParameterValueOnMaterials` _skeletalmesh "HueShift" (`self.ColorVariable`))
  (`MeshComponent.SetScalarParameterValueOnMaterials` (`self.RobotArmStand`) "HueShift" (`self.ColorVariable`))
  (`MeshComponent.SetScalarParameterValueOnMaterials` _skeletalmesh "Saturation" (`self.SaturationValue`))
  (`MeshComponent.SetScalarParameterValueOnMaterials` (`self.RobotArmStand`) "Saturation" (`self.SaturationValue`))
  (`MeshComponent.SetScalarParameterValueOnMaterials` _statelightmesh "Light1On" (select `int` _lightstate :`0` 0.0 :`1` 1.0 :`2` 0.0 :`3` 0.0 :`4` 1.0 :!type "Float (single-precision)"))
  (`MeshComponent.SetScalarParameterValueOnMaterials` _statelightmesh "Light2On" (select `int` _lightstate :`0` 0.0 :`1` 0.0 :`2` 1.0 :`3` 0.0 :`4` 1.0 :!type "Float (single-precision)"))
  (`MeshComponent.SetScalarParameterValueOnMaterials` _statelightmesh "Light3On" (select `int` _lightstate :`0` 0.0 :`1` 0.0 :`2` 0.0 :`3` 1.0 :`4` 1.0 :!type "Float (single-precision)")))