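; BP_Clock_Child is a clock Blueprint variant that shows the seconds of the current time on its TextSec text.
; After the parent BeginPlay, it loops on a 0.2-second Delay, writing the current second as two digits through RefreshSecText.
; It defines CERefreshColonText as an intentional no-op, and its construction script only calls the parent.
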(event `self.ReceiveBeginPlay`
  (`parent.ReceiveBeginPlay`)
  (`self.RefreshSecText` :!label _label)
  (`KismetSystemLibrary.Delay` 0.2)
  (goto _label))

(event `RefreshSecText`
  (`TextRenderComponent.K2_SetText` (`self.TextSec`) (`KismetTextLibrary.Conv_IntToText` (`.Second` (`KismetMathLibrary.BreakDateTime` (`KismetMathLibrary.Now`))) false true 2 2)))

(event `self.CE_RefreshColonText`
  ;[1 1 1] Do Nothing
)

(fn `UserConstructionScript`
  (`parent.UserConstructionScript`))