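; BP_Clock is a digital clock that displays the current system time as two-digit hour and minute text with a blinking colon.
; From BeginPlay, a self-repeating Delay loop calls three custom events every 0.2 seconds to refresh the colon, minute and hour texts.
; Hour and minute are read from Now, while a FlipFlop alternates the colon between visible and empty on each pass.
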(event `self.ReceiveBeginPlay`
  (`self.CE_RefreshColonText` :!label _label)
  (`self.CE_RefreshMinuteText`)
  (`self.CE_RefreshHourText`)
  (`KismetSystemLibrary.Delay` 0.2)
  (goto _label))

(event `CE_RefreshColonText`
  (bind _isa (`/Engine/EditorBlueprintResources/StandardMacros.FlipFlop`)
    (:`A`
      _)
    (:`B`
      _))
  (`TextRenderComponent.K2_SetText` (`self.TextColon`) (select `bool` _isa :`false` " " :`true` ":")))

(event `CE_RefreshHourText`
  (`TextRenderComponent.K2_SetText` (`self.TextHour`) (`KismetTextLibrary.Conv_IntToText` (`.Hour` (`KismetMathLibrary.BreakDateTime` (`KismetMathLibrary.Now`))) false true 2 2)))

(event `CE_RefreshMinuteText`
  (`TextRenderComponent.K2_SetText` (`self.TextMinute`) (`KismetTextLibrary.Conv_IntToText` (`.Minute` (`KismetMathLibrary.BreakDateTime` (`KismetMathLibrary.Now`))) false true 2 2)))

(fn `UserConstructionScript`)