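; BP_Timer is a countdown timer that shows remaining minutes and seconds on text components named TextHour and TextMinute.
; StartTimer sets the time and opens a Gate that lets Tick count down to zero, while StopTimer closes it.
; A looping 0.2-second Delay from BeginPlay refreshes both texts and, while time remains above zero, toggles digit and colon visibility through a FlipFlop to blink.
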(event `self.ReceiveBeginPlay`
  (`self.CE_RefreshHourText` :!label _label)
  (`self.CE_RefreshMinuteText`)
  (if (not (<= (`self.Time`) 0.0))
    (`self.BlinkText`))
  (`KismetSystemLibrary.Delay` 0.2)
  (goto _label))

(event `self.ReceiveTick`
  (params (DeltaSeconds :type "Float (single-precision)"))
  (`/Engine/EditorBlueprintResources/StandardMacros.Gate` false :!label _label_2
    (:`Exit`
      (set `self.Time` (`KismetMathLibrary.FMax` (- (`self.Time`) DeltaSeconds))))))

(event `Start Timer`
  (params (InitialTimeInput :type "Float (double-precision)"))
  (set `self.Time` InitialTimeInput)
  (goto _label_2 :!via `Open`))

(event `Stop Timer`
  (goto _label_2 :!via `Close`))

(event `BlinkText`
  (bind _isa (`/Engine/EditorBlueprintResources/StandardMacros.FlipFlop`)
    (:`A`
      _)
    (:`B`
      _))
  (`SceneComponent.SetVisibility` (`self.TextHour`) _isa false)
  (`SceneComponent.SetVisibility` (`self.TextMinute`) _isa false)
  (`SceneComponent.SetVisibility` (`self.TextColon`) _isa false))

(event `self.CE_RefreshHourText`
  (`TextRenderComponent.K2_SetText` (`self.TextHour`) (`KismetTextLibrary.Conv_IntToText` (`KismetMathLibrary.FTrunc` (/ (`self.Time`) 60.0)) false true 2 2)))

(event `self.CE_RefreshMinuteText`
  (`TextRenderComponent.K2_SetText` (`self.TextMinute`) (`KismetTextLibrary.Conv_IntToText` (`KismetMathLibrary.FTrunc` (mod (`self.Time`) 60.0)) false true 2 2)))

(fn `UserConstructionScript`
  (`parent.UserConstructionScript`))