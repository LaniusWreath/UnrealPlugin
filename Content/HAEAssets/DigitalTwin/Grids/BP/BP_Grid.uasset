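; BP_Grid is a grid actor that builds a field of tiles from one instanced static mesh in its construction script.
; SpawnGrid pulls the mesh, border material and mesh size for the chosen shape from DT_GridShape, then adds scaled instances in local space.
; Both loops use the X tile count, and the corner offsets from its own stored value, leaving the center location unused in placement.
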(fn `GetCurrentShapeData`
  (returns (ShapeDataStruct :type "/SmartFactory/HAEAssets/DigitalTwin/Grids/GridDatas/STRT_GridData Structure"))
  (bind _returnvalue (`|GetDataTableRow` "/SmartFactory/HAEAssets/DigitalTwin/Grids/GridDatas/DT_GridShape.DT_GridShape" (`KismetStringLibrary.Conv_StringToName` (`KismetStringLibrary.Conv_ByteToString` (`self.Grid Shape`))))
    (:`then`
      (return _returnvalue))))

(fn `SpawnGrid`
  (params (CenterLocation :type "Vector Structure") (TileSize :type "Vector Structure") (TileCount :type "Vector2D Structure") (GridShape :type "/SmartFactory/HAEAssets/DigitalTwin/Grids/GridDatas/E_GridShape Enum" :default "NewEnumerator0"))
  (locals (X :type Integer) (Y :type Integer) (TileTransform :type "Transform Structure"))
  (bind _instancedstaticmesh (`self.InstancedStaticMesh`))
  (bind _gridtilecount_x (`KismetMathLibrary.BreakVector2D` (`self.GridTileCount`)))
  (bind _gridtilecount_x_2 (`KismetMathLibrary.BreakVector2D` (`self.GridTileCount`)))
  (bind (_meshsize _mesh _meshmaterial _flatmesh _flatboardermaterial) (break `/SmartFactory/HAEAssets/DigitalTwin/Grids/GridDatas/STRT_GridData` (`self.GetCurrentShapeData`)))
  (set `self.GridCenterLocation` CenterLocation)
  (set `self.GridTileSize` TileSize)
  (set `self.GridTileCount` TileCount)
  (set `self.Grid Shape` GridShape)
  (`StaticMeshComponent.SetStaticMesh` _instancedstaticmesh _flatmesh)
  (`PrimitiveComponent.SetMaterial` _instancedstaticmesh 0 _flatboardermaterial)
  (set `self.GridBottomLeftCornerLocation` (- (`self.GridBottomLeftCornerLocation`) (* (/ (`self.GridTileCount`) (2.0 2.0)) (`self.GridTileSize`))))
  (for _index (range (`KismetMathLibrary.Round` _gridtilecount_x_2))
    (set `local.X` _index)
    (for _index_2 (range (`KismetMathLibrary.Round` _gridtilecount_x))
      (set `local.Y` _index_2)
      (set `local.TileTransform` (`KismetMathLibrary.MakeTransform` (+ (`self.GridBottomLeftCornerLocation`) (* (`self.GridTileSize`) (`KismetMathLibrary.MakeVector` (`KismetMathLibrary.Conv_IntToDouble` (`local.X`)) (`KismetMathLibrary.Conv_IntToDouble` (`local.Y`))))) (struct) (/ (`self.GridTileSize`) (`.MeshSize_2_9CB4AA534A8DD669BB9009B07DF53149` (break `/SmartFactory/HAEAssets/DigitalTwin/Grids/GridDatas/STRT_GridData` (`self.GetCurrentShapeData`))))))
      (`InstancedStaticMeshComponent.AddInstance` (`self.InstancedStaticMesh`) (`local.TileTransform`) false))))

(fn `UserConstructionScript`
  (`self.SpawnGrid` (`self.GridCenterLocation`) (`self.GridTileSize`) (`self.GridTileCount`) (`self.Grid Shape`)))