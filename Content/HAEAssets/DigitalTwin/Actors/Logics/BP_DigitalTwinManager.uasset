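; Digital twin manager Blueprint that bootstraps the twin's HTTP, AGV data and widget managers on BeginPlay.
; A Sequence creates the HTTP manager first, then the AGV data manager, and calls InitializeVehiclePawn on the WebSocket actor with both manager references.
; It then creates the widget manager, initializing it with the first player controller and setting up its member widgets.
; The AGV and widget manager references are assigned None rather than the created instances.
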(event `self.ReceiveBeginPlay`
  (`|ExecutionSequence`
    (:`then_0`
      (bind _returnvalue (`SFCHttpManager.CreateHttpManagerInstance` self))
      (bind (_output_get _output_get_2) (set `self.HttpManagerRef` _returnvalue)))
    (:`then_1`
      (bind _returnvalue_2 (`self.CreateAGVDataManagerInstance` self))
      (bind (_output_get_3 _output_get_4) (set `self.AGVDataManager Ref` null _returnvalue_2))
      (`self.Initialize VehiclePawn` (`.WebSocketActorRef` (`self.WebSocketActorRef`)) _output_get_2 _output_get_4))
    (:`then_2`
      (bind _returnvalue_3 (`self.CreateWidgetManagerInstance` self))
      (bind _asbp_dtwidget_manager (cast `` _returnvalue_3))
      (`/Engine/EditorBlueprintResources/StandardMacros.IsValid` _asbp_dtwidget_manager
        (:`Is Valid`
          (bind (_output_get_5 _output_get_6) (set `self.WidgetManager Ref` null _asbp_dtwidget_manager))
          (`self.InitializeWidgetManager` _output_get_6 (`GameplayStatics.GetPlayerController` 0))
          (`self.InitializeMemberWidgets` _output_get_6))))))

(fn `UserConstructionScript`)