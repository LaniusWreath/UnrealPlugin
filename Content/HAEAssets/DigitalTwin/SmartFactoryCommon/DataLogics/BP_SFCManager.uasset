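; BP_SFCManager is a manager for the SmartFactoryCommon digital twin that bootstraps the UI and offers a data update helper.
; On BeginPlay it creates and stores a BP_SFCWidgetManager, hands it the first player controller, initializes its member widgets and shows the "Main" widget.
; UpdateDataContainer writes a key, value and attributes into a given data container, then prints the resulting attribute map for debugging.
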(event `self.ReceiveBeginPlay`
  (bind _widgetmanagerref (`self.WidgetManagerRef`))
  ;[0.1448 0.1448 0.1448] Initialize Widget Manager Routine
  (bind _returnvalue (`SFCWidgetManager.CreateWidgetManagerInstance` self "/SmartFactory/HAEAssets/DigitalTwin/SmartFactoryCommon/Widgets/BP_SFCWidgetManager.BP_SFCWidgetManager_C"))
  (bind _asbp_sfcwidget_manager (cast `/SmartFactory/HAEAssets/DigitalTwin/SmartFactoryCommon/Widgets/BP_SFCWidgetManager` _returnvalue))
  (`/Engine/EditorBlueprintResources/StandardMacros.IsValid` _asbp_sfcwidget_manager
    (:`Is Valid`
      (set `self.WidgetManagerRef` _asbp_sfcwidget_manager)
      (`SFCWidgetManager.SetPlayerControllerRef` _widgetmanagerref (`GameplayStatics.GetPlayerController` 0))
      (`/SmartFactory/HAEAssets/DigitalTwin/SmartFactoryCommon/Widgets/BP_SFCWidgetManager.InitializeMemberWidgets` _widgetmanagerref)
      (`SFCWidgetManager.ShowWidget` _widgetmanagerref "Main"))))

(fn `UpdateDataContainer`
  (params (TargetDataContainer :type "SFCDataContainer Object Reference") (InputData_Key :type String) (InputData_Value :type String) (InputData_Attributes :type "Map of String to String"))
  (bind _returnvalue (`SFCDataContainer.SetData` TargetDataContainer (make `GenericData` InputData_Key InputData_Value InputData_Attributes)))
  (bind (_returnvalue_key _returnvalue_value _returnvalue_attributes) (break `GenericData` (`SFCDataContainer.GetData` _returnvalue)))
  (`SFCDataManageUtilities.PrintStringMapMembers` _returnvalue_attributes 5.0 (struct :`G` 255 :`A` 255)))

(fn `UserConstructionScript`)