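; BP_StopWatch is a stopwatch actor that displays elapsed time as two-digit seconds and hundredths.
; StartWatch stores a time limit, resets the time and opens a Tick gate that accumulates delta seconds and refreshes both texts; StopWatch closes it.
; Despite their names, TextHour shows seconds capped at the limit and TextMinute shows hundredths, zeroed from a hard-coded 60 seconds.
; Reaching the limit does not stop the count.
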(event `self.ReceiveBeginPlay`
  ;[1 1 1] Do Nothing
)

(event `self.ReceiveTick`
  (params (DeltaSeconds :type "Float (single-precision)"))
  (`/Engine/EditorBlueprintResources/StandardMacros.Gate` true :!label _label
    (:`Exit`
      (set `self.Time` (+ (`self.Time`) DeltaSeconds))
      (`self.CE_RefreshHourText`)
      (`self.CE_RefreshMinuteText`))))

(event `StartWatch`
  (params (`Time Limit` :type "Float (double-precision)"))
  (set `self.Time Limit` `Time Limit`)
  (set `self.Time` 0.0)
  (goto _label :!via `Open`))

(event `StopWatch`
  (goto _label :!via `Close`))

(event `self.CE_RefreshHourText`
  (`TextRenderComponent.K2_SetText` (`self.TextHour`) (`KismetTextLibrary.Conv_IntToText` (`KismetMathLibrary.Min` (`KismetMathLibrary.FTrunc` (`self.Time`)) (`KismetMathLibrary.FTrunc` (`self.Time Limit`))) false false 2 2)))

(event `self.CE_RefreshMinuteText`
  (bind _time (`self.Time`))
  (`TextRenderComponent.K2_SetText` (`self.TextMinute`) (`KismetTextLibrary.Conv_IntToText` (`KismetMathLibrary.SelectInt` 0 (`KismetMathLibrary.FTrunc` (* (mod _time 1.0) 100.0)) (>= _time 60.0)) false false 2 2)))

(fn `UserConstructionScript`
  (`parent.UserConstructionScript`))