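; Analog clock actor with a click-toggled alarm, showing the system's current time.
; A looping one-second timer rotates the hour, minute and second scene components from Now(), with fractional hour and minute positions.
; A second timer prints "Alarm" each second for about five minutes from the set time while enabled.
; Clicking the actor toggles the alarm and moves its button; BeginPlay enables the cursor and click events.
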(event `self.ReceiveBeginPlay`
  (bind _returnvalue (`GameplayStatics.GetPlayerController` 0))
  (set `PlayerController.bShowMouseCursor` true _returnvalue)
  (set `PlayerController.bEnableClickEvents` true _returnvalue)
  (`KismetSystemLibrary.K2_SetTimerDelegate` (delegate `RefreshNeedles`) 1.0 true)
  (`KismetSystemLibrary.K2_SetTimerDelegate` (delegate `CheckForAlarm`) 1.0 true))

(event `RefreshNeedles`
  (`self.RefreshHourNeedle`)
  (`self.RefreshSecNeedle`)
  (`self.RefreshMinuteNeedle`))

(event `CheckForAlarm`
  (bind (_year _month _day _hour _minute) (`KismetMathLibrary.BreakDateTime` (`KismetMathLibrary.Now`)))
  (bind _returnvalue (+ (`KismetMathLibrary.Conv_IntToDouble` (`self.AlarmHour`)) (/ (`KismetMathLibrary.Conv_IntToDouble` (`self.AlarmMinute`)) 60.0)))
  (bind _returnvalue_2 (+ (`KismetMathLibrary.Conv_IntToDouble` _hour) (/ (`KismetMathLibrary.Conv_IntToDouble` _minute) 60.0)))
  ;[1 1 1] Alarm
  (if (and (>= _returnvalue_2 _returnvalue) (< (- _returnvalue_2 _returnvalue) 0.083333) (`self.IsAlarmOn`))
    (`KismetSystemLibrary.PrintString` "Alarm")))

(event `EnableAlarm`
  ;[1 1 1] AlarmToggle
  (`SceneComponent.K2_SetRelativeLocation` (`self.AlarmButton`) (0.0 0.0 67.0) false false)
  (set `self.IsAlarmOn` true))

(event `RefreshHourNeedle`
  (bind (_year _month _day _hour _minute) (`KismetMathLibrary.BreakDateTime` (`KismetMathLibrary.Now`)))
  ;[1 1 1] Needle
  (`SceneComponent.K2_SetRelativeRotation` (`self.HourScene`) (`KismetMathLibrary.MakeRotator` (* (+ (`KismetMathLibrary.Conv_IntToDouble` (mod _hour 12)) (/ (`KismetMathLibrary.Conv_IntToDouble` _minute) 60.0)) -30.0)) false false))

(event `DissableAlarm`
  ;[1 1 1] AlarmToggle
  (`SceneComponent.K2_SetRelativeLocation` (`self.AlarmButton`) (0.0 0.0 72.0) false false)
  (set `self.IsAlarmOn` false))

(event `RefreshMinuteNeedle`
  (bind (_year _month _day _hour _minute _second) (`KismetMathLibrary.BreakDateTime` (`KismetMathLibrary.Now`)))
  ;[1 1 1] Needle
  (`SceneComponent.K2_SetRelativeRotation` (`self.MinuteScene`) (`KismetMathLibrary.MakeRotator` (* (+ (`KismetMathLibrary.Conv_IntToDouble` _minute) (/ (`KismetMathLibrary.Conv_IntToDouble` _second) 60.0)) -6.0)) false false))

(event `self.ReceiveActorOnClicked`
  (params (ButtonPressed :type "Key Structure"))
  ;[1 1 1] AlarmToggle
  ;;[1 1 1] 코멘트
  (if (`self.IsAlarmOn`)
    (`self.DissableAlarm`)
    (else
      (`self.EnableAlarm`))))

(event `RefreshSecNeedle`
  ;[1 1 1] Needle
  (`SceneComponent.K2_SetRelativeRotation` (`self.SecScene`) (`KismetMathLibrary.MakeRotator` (* (`KismetMathLibrary.Conv_IntToDouble` (`.Second` (`KismetMathLibrary.BreakDateTime` (`KismetMathLibrary.Now`)))) -6.0)) false false))

(fn `UserConstructionScript`)