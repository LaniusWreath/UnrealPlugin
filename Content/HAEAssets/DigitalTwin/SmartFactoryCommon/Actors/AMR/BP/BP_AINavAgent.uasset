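; BP_AINavAgent is an AI-navigated AMR pawn for the smart factory digital twin that cycles through a list of target actors.
; From BeginPlay, StartMovementCall issues AIMoveTo to the current target, advances the wrapping index and re-calls itself after a short delay.
; The loop follows the immediate exec output, so it retargets without waiting for arrival.
; An unconnected random-point wander loop never runs.
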(event `self.ReceiveBeginPlay`
  (`self.StartMovementCall`))

(event `StartMovementCall`
  (`|AIMoveTo` self (`self.K2_GetActorLocation` (`|GetArrayItem` (`self.TargetActors`) (`self.TargetIndex`))) null 0.0
    (:`then`
      (set `self.TargetIndex` (mod (+ (`self.TargetIndex`) 1) (`KismetArrayLibrary.Array_Length` (`self.TargetActors`))))
      (`KismetSystemLibrary.Delay` 1.0)
      (`self.StartMovementCall`))))

(fn `UserConstructionScript`)