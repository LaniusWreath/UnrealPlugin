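; AI navigation agent for an AMR that travels between stops in a TargetActors list using AIMoveTo.
; CallMoveAMR passes TargetIndex to MoveAMR, which heads for that target's AMRPlacer and records CurrentIndex on success.
; StartMovementCall cycles through target actor locations, advancing after a short delay without waiting for arrival.
; BeginPlay is empty, and a random-wander loop is left unconnected.
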(event `CallMoveAMR`
  (`/SmartFactory/Seungwoo/AMR/BP/BPIF_AMR.MoveAMR` (`self.TargetIndex`)))

(event `/SmartFactory/Seungwoo/AMR/BP/BPIF_AMR.MoveAMR`
  (params (TargetIndex :type Integer))
  (`|AIMoveTo` self (`SceneComponent.K2_GetComponentLocation` (`/SmartFactory/Seungwoo/Cell/BP_Cell.AMRPlacer` (`|GetArrayItem` (`self.TargetActors`) TargetIndex))) null 1.0
    (:`OnSuccess`
      (set `self.CurrentIndex` TargetIndex))))

(event `self.ReceiveBeginPlay`)

(event `StartMovementCall`
  (`|AIMoveTo` self (`self.K2_GetActorLocation` (`|GetArrayItem` (`self.TargetActors`) (`self.TargetIndex`))) null 0.0
    (:`then`
      (set `self.TargetIndex` (mod (+ (`self.TargetIndex`) 1) (`KismetArrayLibrary.Array_Length` (`self.TargetActors`))))
      (`KismetSystemLibrary.Delay` 1.0)
      (`self.StartMovementCall`))))

(fn `UserConstructionScript`)