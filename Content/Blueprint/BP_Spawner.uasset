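; Spawner actor that periodically creates BP_SpawnedObject items and sends them moving along a path spline toward rack storage.
; BeginPlay positions the spawn point and starts a looping timer, whose random interval is picked once rather than per spawn.
; Each spawn is scaled down, rotated, given a random rack Row and Col, then handed PathSpline through SetMovingFlag.
; A separate SpawnObject function repeats this without rack data and is not called here.
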(event `self.ReceiveBeginPlay`
  ;[1 1 1] Get Spawn Location
  (`SceneComponent.K2_SetRelativeLocation` (`self.SpawnLocationRef`) (`self.SpawnLocation`) false false)
  (`KismetSystemLibrary.K2_SetTimerDelegate` (delegate `Spawn`) (`KismetMathLibrary.Conv_IntToDouble` (`KismetMathLibrary.RandomIntegerInRange` 2 7)) true))

(event `Spawn`
  (bind _returnvalue (`|SpawnActorFromClass` "/SmartFactory/Blueprint/BP_SpawnedObject.BP_SpawnedObject_C" (`KismetMathLibrary.MakeTransform` (`SceneComponent.K2_GetComponentLocation` (`self.SpawnLocationRef`)) (struct :`Yaw` -90.0) (* (1.0 1.0 1.0) 0.6)) "Undefined" "MultiplyWithRoot" null (`KismetMathLibrary.RandomIntegerInRange` 0 6) (`KismetMathLibrary.RandomIntegerInRange` 1 6) null))
  (bind _output_get (set `self.SpawnedObject` _returnvalue))
  ;[1 1 1] Return Path Info to BP_Spawned Object
  (`/SmartFactory/Blueprint/BP_SpawnedObject.SetMovingFlag` _output_get true (`self.PathSpline`)))

(fn `SpawnObject`
  (bind _returnvalue (`|SpawnActorFromClass` "/SmartFactory/Blueprint/BP_SpawnedObject.BP_SpawnedObject_C" (`KismetMathLibrary.MakeTransform` (`SceneComponent.K2_GetComponentLocation` (`self.SpawnLocationRef`))) "Undefined" "MultiplyWithRoot" null 0 0 null))
  (bind _output_get (set `self.SpawnedObject` _returnvalue))
  (`/SmartFactory/Blueprint/BP_SpawnedObject.SetMovingFlag` _output_get true (`self.PathSpline`)))

(fn `UserConstructionScript`)