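; BP_PaintRobot is a paint robot arm facility that mirrors server-reported equipment data in the scene.
; Activating it sends an HTTP GET keyed by its facility ID and starts the skeletal work animation, effect and environment audio, which stopping turns off.
; Responses update a WBP_Facility widget with arm ID, recent start time, operating status, electric current and fever, read from the data container.
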(event `self.ReceiveBeginPlay`
  (`|ExecutionSequence`
    (:`then_0`
      (`self.InitializeDataManagers`)
      (bind _aswbp_facility (cast `/SmartFactory/Widget/khy/WBP_Facility` (`WidgetComponent.GetUserWidgetObject` (`self.Widget`))))
      (set `self.FacilityWeidgetRef` _aswbp_facility))
    (:`then_1`
      (bind _ass_industrial_robot_skeleton_anim_blueprint (cast `/SmartFactory/SkeletalMesh/S_IndustrialRobot_Skeleton_AnimBlueprint` (`SkeletalMeshComponent.GetAnimInstance` (`self.SkeletalMesh`))))
      (set `self.ABP_SkeletonRef` _ass_industrial_robot_skeleton_anim_blueprint))))

(event `Stop`
  ;[1 1 1] Operate
  (`/SmartFactory/Widget/khy/WBP_Facility.ReturnWidget` (`self.FacilityWeidgetRef`))
  (set `self.bWorking` false)
  (set `/SmartFactory/SkeletalMesh/S_IndustrialRobot_Skeleton_AnimBlueprint.StartWork` false (`self.ABP_SkeletonRef`))
  (`ActorComponent.Deactivate` (`self.Effect`))
  (`ActorComponent.Deactivate` (`self.EnvironmentAudio`)))

(event `Operate`
  ;[1 1 1] Operate
  (`self.MakeGetRequest`)
  (set `self.bWorking` true)
  (set `/SmartFactory/SkeletalMesh/S_IndustrialRobot_Skeleton_AnimBlueprint.StartWork` true (`self.ABP_SkeletonRef`))
  (`ActorComponent.Activate` (`self.Effect`) true)
  (`ActorComponent.Activate` (`self.EnvironmentAudio`) true))

(fn `ActivateFacility`
  (`parent.ActivateFacility`)
  (`self.Operate`))

(fn `GetActorData`
  (returns (OutActorData :type "/SmartFactory/Blueprint/Logics/STRT_ActorData Structure"))
  (return))

(fn `MakeGetRequest`
  (`SFCHttpManager.MakeGetRequestWithHeader` (`self.HTTPManagerRef`) (`self.Url`) (`|MakeMap` "accept" "application/json") (`|MakeMap` "robotArmId" (`self.FacilityID`)) true))

(fn `OnHTTPResponseReceived`
  (bind (_returnvalue_key _returnvalue_value _returnvalue_attributes) (break `GenericData` (`SFCDataContainer.GetData` (`self.DataContainerRef`))))
  (bind (_robotarmid _recentstarttime _processtime _operatingstatus _fever _electriccurrent) (`/SmartFactory/Blueprint/Logics/BPFL_EquipmentDataParsing.FindFacilityDataFromMap` _returnvalue_attributes))
  (`parent.OnHTTPResponseReceived`)
  (`/SmartFactory/Widget/khy/WBP_Facility.UpdateRobotArmWidgetData` (`self.FacilityWeidgetRef`) (`KismetTextLibrary.Conv_StringToText` _robotarmid) (`KismetTextLibrary.Conv_StringToText` (`KismetStringLibrary.GetSubstring` _recentstarttime 11 8)) (`KismetTextLibrary.Conv_StringToText` _operatingstatus) (`KismetStringLibrary.Conv_StringToDouble` _electriccurrent) (`KismetStringLibrary.Conv_StringToDouble` _fever)))

(fn `SetServerURL`
  (params (InUrl :type String) (InFacilityID :type String))
  (`parent.SetServerURL` InUrl InFacilityID))

(fn `StopFacility`
  (`parent.StopFacility`)
  (`self.Stop`))

(fn `UserConstructionScript`)