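; Selectable welding robot arm facility for a smart factory scene, which animates while operating and shows server data on its widget.
; A gated Tick moves a target through looping waypoints, yawing the stand and passing the point to the AnimInstance.
; Operation state switches the gate, lights, audio and sparks, and updates the GameMode's text when selected.
; Operate and Stop also send HTTP GET requests, whose responses refresh the facility widget.
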(event `self.ReceiveBeginPlay`
  (`self.InitializeDataManagers`)
  (bind _aswbp_facility (cast `/SmartFactory/Widget/khy/WBP_Facility` (`WidgetComponent.GetUserWidgetObject` (`self.Widget`))))
  (set `self.FacilityWeidgetRef` _aswbp_facility))

(event `self.ReceiveTick`
  (params (DeltaSeconds :type "Float (single-precision)"))
  ;[1 1 1] Animation
  (`/Engine/EditorBlueprintResources/StandardMacros.Gate` true :!label _label
    (:`Exit`
      (set `self.TargetLocation` (+ (`self.TargetLocation`) (* (* (`KismetMathLibrary.Normal` (- (`|GetArrayItem` (`self.LocationList`) (`self.LocationIndex`)) (`self.TargetLocation`))) (`self.MovementSpeed`)) DeltaSeconds)))
      (if (< (`KismetMathLibrary.Vector_Distance` (`self.TargetLocation`) (`|GetArrayItem` (`self.LocationList`) (`self.LocationIndex`))) (* (`self.MovementSpeed`) DeltaSeconds))
        (set `self.TargetLocation` (`|GetArrayItem` (`self.LocationList`) (`self.LocationIndex`)))
        (set `self.LocationIndex` (mod (+ (`self.LocationIndex`) 1) (`KismetArrayLibrary.Array_Length` (`self.LocationList`)))))
      (`self.RefreshTargetLocation`))))

(event `OpenTickGate`
  ;[1 1 1] Animation
  (goto _label :!via `Open`))

(event `CloseTickGate`
  ;[1 1 1] Animation
  (goto _label :!via `Close`))

(event `RefreshTargetLocation`
  ;[1 1 1] Movement
  (`SceneComponent.K2_SetRelativeLocation` (`self.LocationReferenceScene`) (+ (`self.TargetLocation`) (0.0 0.0 75.0)) false false)
  (`SceneComponent.K2_SetRelativeRotation` (`self.RobotArmStand`) (`KismetMathLibrary.MakeRotator` 0.0 0.0 (- (.yaw (`KismetMathLibrary.FindLookAtRotation` (`SceneComponent.K2_GetComponentLocation` (`self.RobotArmStand`)) (`SceneComponent.K2_GetComponentLocation` (`self.LocationReferenceScene`)))) (`KismetMathLibrary.DegAsin` (/ 20.0 (`KismetMathLibrary.Vector_Distance` (`SceneComponent.K2_GetComponentLocation` (`self.LocationReferenceScene`)) (`SceneComponent.K2_GetComponentLocation` (`self.RobotArmStand`))))))) false false)
  (message `/SmartFactory/Blueprint/Logics/BPIF_AnimControl.SetVectorData` (`SkeletalMeshComponent.GetAnimInstance` (`self.SkeletalMesh`)) (.location (`KismetMathLibrary.MakeRelativeTransform` (`SceneComponent.K2_GetComponentToWorld` (`self.LocationReferenceScene`)) (`SceneComponent.K2_GetComponentToWorld` (`self.SkeletalMesh`)))) "TargetLocation"))

(event `SetNewOperationState`
  (params (InOperationState :type "/SmartFactory/Blueprint/Logics/Enum_OperationState Enum" :default "NewEnumerator0"))
  ;[1 1 1] OperationState
  (bind _output_get (set `self.OperationState` InOperationState))
  (bind _structout (setmembers `/SmartFactory/Blueprint/Logics/STRT_ActorData` :`StructRef` (`self.ActorData`) :`OperationState` _output_get))
  (set `self.ActorData` _structout)
  (bind _asgame_mode_smart_factory_base (cast `/SmartFactory/Blueprint/Logics/GameMode_SmartFactoryBase` (`GameplayStatics.GetGameMode`)))
  (if (== (`/SmartFactory/Blueprint/Logics/GameMode_SmartFactoryBase.CurrentSelectedActor` _asgame_mode_smart_factory_base) self)
    (`/SmartFactory/Blueprint/Logics/GameMode_SmartFactoryBase.SetWidgetText` _asgame_mode_smart_factory_base (`self.ActorData`)))
  (switch `/SmartFactory/Blueprint/Logics/Enum_OperationState` (`self.OperationState`)
    (:`NewEnumerator0`
      (`|ExecutionSequence`
        (:`then_0`
          (`MeshComponent.SetScalarParameterValueOnMaterials` (`self.SphereLight1`) "Intensity" 0.0)
          (`MeshComponent.SetScalarParameterValueOnMaterials` (`self.SphereLight2`) "Intensity" 0.0)
          (set `self.LightState` 1))
        (:`then_1`
          (`self.CloseTickGate`))
        (:`then_2`
          (`ActorComponent.Deactivate` (`self.EnvironmentAudio`))
          (`self.DeactivateWeldSparkConsist`))))
    (:`NewEnumerator1`
      (`|ExecutionSequence`
        (:`then_0`
          (`MeshComponent.SetScalarParameterValueOnMaterials` (`self.SphereLight1`) "Intensity" 100.0)
          (`MeshComponent.SetScalarParameterValueOnMaterials` (`self.SphereLight2`) "Intensity" 100.0)
          (set `self.LightState` 3))
        (:`then_1`
          (`self.OpenTickGate`))
        (:`then_2`
          (`ActorComponent.Activate` (`self.EnvironmentAudio`) true)
          (`self.ActivateWeldSparkConsist`))))))

(event `self.ReceiveActorOnClicked`
  (params (ButtonPressed :type "Key Structure"))
  ;[1 1 1] Select
  (`self.OnActorSelected`))

(event `/SmartFactory/Blueprint/Logics/BPIF_SelectableActor.OnActorSelected`
  ;[1 1 1] Select
  (bind _asgame_mode_smart_factory_base (cast `/SmartFactory/Blueprint/Logics/GameMode_SmartFactoryBase` (`GameplayStatics.GetGameMode`)))
  (`/SmartFactory/Blueprint/Logics/GameMode_SmartFactoryBase.OnSelectableActorClicked` _asgame_mode_smart_factory_base self))

(event `/SmartFactory/Blueprint/Logics/BPIF_SelectableActor.EnableSelection`
  ;[1 1 1] Select
  (`SceneComponent.SetVisibility` (`self.SelectionPlane`) true false)
  (bind _asgame_mode_smart_factory_base (cast `/SmartFactory/Blueprint/Logics/GameMode_SmartFactoryBase` (`GameplayStatics.GetGameMode`)))
  (`/SmartFactory/Blueprint/Logics/GameMode_SmartFactoryBase.SetWidgetText` _asgame_mode_smart_factory_base (`self.ActorData`)))

(event `/SmartFactory/Blueprint/Logics/BPIF_SelectableActor.DisableSelection`
  ;[1 1 1] Select
  (`SceneComponent.SetVisibility` (`self.SelectionPlane`) false false))

(event `Operate`
  ;[1 1 1] Operate
  (`self.SetNewOperationState` "NewEnumerator1")
  (`self.MakeGetRequest`))

(event `Stop`
  ;[1 1 1] Operate
  (`self.SetNewOperationState` "NewEnumerator0")
  (`self.MakeGetRequest`))

(event `DeactivateWeldSparkConsist`
  (`ActorComponent.Deactivate` (`self.Effect_WeldSparkConsist`)))

(event `ActivateWeldSpark`
  (`ActorComponent.Activate` (`self.Effect_WeldSpark`) true))

(event `ActivateWeldSparkConsist`
  (`ActorComponent.Activate` (`self.Effect_WeldSparkConsist`) false))

(fn `ActivateFacility`
  (`parent.ActivateFacility`)
  (`self.Operate`))

(fn `GetActorData`
  (returns (OutActorData :type "/SmartFactory/Blueprint/Logics/STRT_ActorData Structure"))
  (return (`self.ActorData`)))

(fn `MakeGetRequest`
  (`SFCHttpManager.MakeGetRequestWithHeader` (`self.HTTPManagerRef`) (`self.Url`) (`|MakeMap` "accept" "application/json") (`|MakeMap` "robotArmId" (`self.FacilityID`)) true))

(fn `OnHTTPResponseReceived`
  (bind (_returnvalue_key _returnvalue_value _returnvalue_attributes) (break `GenericData` (`SFCDataContainer.GetData` (`self.DataContainerRef`))))
  (bind (_robotarmid _recentstarttime _processtime _operatingstatus _fever _electriccurrent) (`/SmartFactory/Blueprint/Logics/BPFL_FacilityDataParsing.FindFacilityDataFromMap` _returnvalue_attributes))
  (`parent.OnHTTPResponseReceived`)
  (`/SmartFactory/Widget/khy/WBP_Facility.UpdateRobotArmWidgetData` (`self.FacilityWeidgetRef`) (`KismetTextLibrary.Conv_StringToText` _robotarmid) (`KismetTextLibrary.Conv_StringToText` (`KismetStringLibrary.GetSubstring` _recentstarttime 11 8)) (`KismetTextLibrary.Conv_StringToText` _operatingstatus) (`KismetStringLibrary.Conv_StringToDouble` _electriccurrent) (`KismetStringLibrary.Conv_StringToDouble` _fever)))

(fn `SetServerURL`
  (params (InUrl :type String) (InFacilityID :type String))
  (`parent.SetServerURL` InUrl InFacilityID))

(fn `StopFacility`
  (`parent.StopFacility`)
  (`self.Stop`))

(fn `UserConstructionScript`
  (bind _skeletalmesh (`self.SkeletalMesh`))
  (`self.RefreshTargetLocation`)
  (`MeshComponent.SetScalarParameterValueOnMaterials` _skeletalmesh "HueShift" (`self.ColorVariable`))
  (`MeshComponent.SetScalarParameterValueOnMaterials` (`self.RobotArmStand`) "HueShift" (`self.ColorVariable`))
  (`MeshComponent.SetScalarParameterValueOnMaterials` _skeletalmesh "Saturation" (`self.SaturationValue`))
  (`MeshComponent.SetScalarParameterValueOnMaterials` (`self.RobotArmStand`) "Saturation" (`self.SaturationValue`)))