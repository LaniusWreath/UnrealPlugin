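; Logistics actor that, once spawned, travels along a spline path handed to it through SetMovingFlag.
; Tick advances a distance by Speed and places the actor at that world point on the spline, applying a fixed tilt past spline input key 4.
; On reaching the spline's end it stops, and while not moving it holds a fixed rotation.
; NewFunction stores a Row and Col on the object.
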(event `self.ReceiveTick`
  (params (DeltaSeconds :type "Float (single-precision)"))
  (if (`self.bMoving`)
    (bind _output_get (set `self.Distance` (+ (* DeltaSeconds (`self.Speed`)) (`self.Distance`))))
    (if (>= _output_get (`SplineComponent.GetSplineLength` (`self.SplineRef`)))
      (set `self.bMoving` false)
      (else
        ;[1 1 1] Move Along Spline
        (`self.K2_SetActorLocation` (* (`SplineComponent.GetLocationAtDistanceAlongSpline` (`self.SplineRef`) _output_get "World") 1.0))
        ;[1 1 1] Set Rotation Offset
        (if (>= _output_get (`SplineComponent.GetDistanceAlongSplineAtSplineInputKey` (`self.SplineRef`) 4.0))
          (`self.K2_SetActorRotation` (struct :`Roll` -40.0)))))
    (else
      (`self.K2_SetActorRotation` (struct :`Yaw` -90.0)))))

(event `SetMovingFlag`
  (params (bMoving :type Boolean) (SplineComponentRef :type "SplineComponent Object Reference"))
  ;[1 1 1] Spawn 완료 후 전달받은 경로 정보 저장하기
  (set `self.bMoving` bMoving)
  (set `self.SplineRef` SplineComponentRef))

(fn `NewFunction`
  (params (row :type Integer) (col :type Integer))
  (set `self.row` row)
  (set `self.col` col))

(fn `UserConstructionScript`)