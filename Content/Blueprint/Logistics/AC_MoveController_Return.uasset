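; Movement controller component that returns a logistics loader from its move target location to its start location.
; Each Move call advances Alpha by MoveSpeed over a fixed 0.016 timestep and passes the linearly interpolated position to the owner's MoveLoader.
; When Alpha reaches 1, it snaps the loader to the start location, then calls EndMovement and InitMovement.
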(event `self.Move`
  (bind _owner (`self.Owner`))
  (bind _owner_2 (`self.Owner`))
  (bind _output_get (set `self.Alpha` (`KismetMathLibrary.FMin` (+ (`self.Alpha`) (* (`self.MoveSpeed`) 0.016)) 1.0)))
  (if (>= _output_get 1.0)
    (`/SmartFactory/Blueprint/BP_RackLoader.MoveLoader` _owner (`/SmartFactory/Blueprint/BP_RackLoader.StartLocation` _owner))
    (`self.EndMovement`)
    (`self.InitMovement`)
    (else
      (`/SmartFactory/Blueprint/BP_RackLoader.MoveLoader` (`self.Owner`) (`KismetMathLibrary.VLerp` (`/SmartFactory/Blueprint/BP_RackLoader.MoveTargetLocation` _owner_2) (`/SmartFactory/Blueprint/BP_RackLoader.StartLocation` _owner_2) (`self.Alpha`))))))