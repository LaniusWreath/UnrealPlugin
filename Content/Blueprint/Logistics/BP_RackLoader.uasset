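; BP_RackLoader is a logistics rack loader that carries boxes on a rail-mounted tray into rack slots.
; On load, it attaches the box, derives the target from its row and column, and starts a movement controller.
; A separate return controller brings it back after unloading, then signals that it can load again.
; MoveLoader positions the clamped vertical rail and tray, also running at construction to preview the current location.
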(event `self.ReceiveBeginPlay`
  ;[1 1 1] When Arriving at the Target Location
  (add `/SmartFactory/Blueprint/Logistics/AC_MoveController.OnMovementEnd` (`self.AC_MoveController`) (`|CreateDelegate` :!event `UnloadBox`))
  ;[1 1 1] When Back at the Initial Location
  (add `/SmartFactory/Blueprint/Logistics/AC_MoveController.OnMovementEnd` (`self.AC_MoveController_Return`) (delegate `EnableLoad`))
  (`ActorComponent.Activate` (`self.MS_Conveyor`) true))

(event `EnableLoad`
  ;[1 1 1] When Back at the Initial Location
  (set `self.bMoving` false)
  (`self.OnMovementEnd`))

(event `OnLoad`
  (params (Box :type "/SmartFactory/Blueprint/Logistics/BP_SpawnedObject Object Reference"))
  (bind _box (`self.Box`))
  ;[1 1 1] Retrieve Box From Queue
  (`ActorComponent.Activate` (`self.Niagara`) true)
  (bind _output_get (set `self.Box` Box))
  (`self.K2_AttachToComponent` _output_get (`self.BoxPosition`) "None" "SnapToTarget" "SnapToTarget" "KeepWorld" true)
  (set `self.MoveTargetLocation` (`KismetMathLibrary.MakeVector` (+ (* 200.0 (`/SmartFactory/Blueprint/Logistics/BP_SpawnedObject.col` _box)) (.x (`self.InitTargetLocation`)) -40.0) (.y (`self.InitTargetLocation`)) (+ (.z (`self.InitTargetLocation`)) (* 106.0 (`/SmartFactory/Blueprint/Logistics/BP_SpawnedObject.row` _box)) -10.0)))
  ;[1 1 1] Move Loader from Initial Location to Target Location
  (set `self.MovementState` (`self.AC_MoveController`))
  (set `self.bMoving` true)
  (`/SmartFactory/Blueprint/Logistics/AC_MoveController.StartMovement` (`self.MovementState`)))

(event `UnloadBox`
  (bind _box (`self.Box`))
  ;[1 1 1] Insert a Box into the Rack
  (`self.K2_AddActorWorldOffset` _box (`self.UnloadBoxDeltaLocation`) false false)
  (`self.K2_DetachFromActor` _box "KeepWorld" "KeepWorld" "KeepWorld")
  ;[1 1 1] Initialize Box Info
  (set `self.Box` null)
  ;[1 1 1] Go Back to the Initial Location
  (set `self.MovementState` (`self.AC_MoveController_Return`))
  (`/SmartFactory/Blueprint/Logistics/AC_MoveController.StartMovement` (`self.MovementState`)))

(event `MoveLoader`
  (params (TargetLocation :type "Vector Structure"))
  (set `self.CurrentLocation` TargetLocation)
  (`SceneComponent.SetRelativeScale3D` (`self.HorizontalLine`) (`KismetMathLibrary.MakeVector` (* (`KismetMathLibrary.VSize` (- (`self.EndLocation`) (`self.StartLocation`))) 0.01) 1.0 1.0))
  (`self.GoToTarget`))

(fn `GoToTarget`
  (`SceneComponent.K2_SetRelativeLocation` (`self.VerticalLine`) (`KismetMathLibrary.MakeVector` (`KismetMathLibrary.FClamp` (.x (`self.CurrentLocation`)) (.x (`self.StartLocation`)) (.x (`self.EndLocation`))) 0.0 400.0) false false)
  (`SceneComponent.K2_SetRelativeLocation` (`self.Tray`) (`KismetMathLibrary.MakeVector` (+ (`KismetMathLibrary.FClamp` (.x (`self.CurrentLocation`)) (.x (`self.StartLocation`)) (.x (`self.EndLocation`))) 25.0) 0.0 (+ (.z (`self.CurrentLocation`)) 40.0)) false false))

(fn `UserConstructionScript`
  (`self.MoveLoader` (`self.CurrentLocation`)))