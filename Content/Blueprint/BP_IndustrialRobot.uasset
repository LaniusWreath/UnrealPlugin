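; BP_IndustrialRobot is an industrial robot Blueprint with events to start and stop its work animation.
; Both events cast the skeletal mesh's anim instance to the robot's Animation Blueprint, setting StartWork or EndWork to true.
; Stopping also deactivates a Niagara effect, which this graph never activates.
; Neither flag is reset here, and the construction script is empty.
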(event `StartRobotWork`
  (bind _ass_industrial_robot_skeleton_anim_blueprint (cast `/SmartFactory/SkeletalMesh/S_IndustrialRobot_Skeleton_AnimBlueprint` (`SkeletalMeshComponent.GetAnimInstance` (`self.SkeletalMesh`))))
  (set `/SmartFactory/SkeletalMesh/S_IndustrialRobot_Skeleton_AnimBlueprint.StartWork` true _ass_industrial_robot_skeleton_anim_blueprint))

(event `StopRobotWork`
  (bind _ass_industrial_robot_skeleton_anim_blueprint (cast `/SmartFactory/SkeletalMesh/S_IndustrialRobot_Skeleton_AnimBlueprint` (`SkeletalMeshComponent.GetAnimInstance` (`self.SkeletalMesh`))))
  (`ActorComponent.Deactivate` (`self.NewNiagaraSystem`))
  (set `/SmartFactory/SkeletalMesh/S_IndustrialRobot_Skeleton_AnimBlueprint.EndWork` true _ass_industrial_robot_skeleton_anim_blueprint))

(fn `UserConstructionScript`)