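; Blueprint function library that converts AMR telemetry between individual fields and a string-keyed map of JSON data.
; A make function packs type, state, destination, location, height, direction, velocity, battery and collision flag into the map.
; Two find functions unpack the same keys, as raw values or as Text for display, without checking that keys exist.
; All three share hardcoded key names, including the misspelled "collisionEtected".
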(fn `FindAMRDatasFromMap_String`
  (params (AMRDataJsonMap :type "Map of String to String (by ref)"))
  (returns (outAMRType :type String) (outState :type String) (outDestination :type String) (outLocationX :type String) (outLocationY :type String) (outLocationZ :type String) (outLocationVelocity :type String) (outLocationBattery :type String) (outCollisionDetected :type String) (height :type String) (direction :type String))
  (return (`BlueprintMapLibrary.Map_Find` AMRDataJsonMap "amrType") (`BlueprintMapLibrary.Map_Find` AMRDataJsonMap "state") (`BlueprintMapLibrary.Map_Find` AMRDataJsonMap "destination") (`BlueprintMapLibrary.Map_Find` AMRDataJsonMap "locationX") (`BlueprintMapLibrary.Map_Find` AMRDataJsonMap "locationY") (`BlueprintMapLibrary.Map_Find` AMRDataJsonMap "locationZ") (`BlueprintMapLibrary.Map_Find` AMRDataJsonMap "velocity") (`BlueprintMapLibrary.Map_Find` AMRDataJsonMap "battery") (`BlueprintMapLibrary.Map_Find` AMRDataJsonMap "collisionEtected") (`BlueprintMapLibrary.Map_Find` AMRDataJsonMap "height") (`BlueprintMapLibrary.Map_Find` AMRDataJsonMap "direction")))

(fn `FindAMRDatasFromMap_TEXT`
  (params (AMRDataJsonMap :type "Map of String to String (by ref)"))
  (returns (outAMRType :type Text) (outState :type Text) (outDestination :type Text) (outLocationX :type Text) (outLocationY :type Text) (outLocationZ :type Text) (outHeight :type Text) (outDirection :type Text) (outLocationVelocity :type Text) (outLocationBattery :type Text) (outCollisionDetected :type Text))
  (return (`KismetTextLibrary.Conv_StringToText` (`BlueprintMapLibrary.Map_Find` AMRDataJsonMap "amrType")) (`KismetTextLibrary.Conv_StringToText` (`BlueprintMapLibrary.Map_Find` AMRDataJsonMap "state")) (`KismetTextLibrary.Conv_StringToText` (`BlueprintMapLibrary.Map_Find` AMRDataJsonMap "destination")) (`KismetTextLibrary.Conv_StringToText` (`BlueprintMapLibrary.Map_Find` AMRDataJsonMap "locationX")) (`KismetTextLibrary.Conv_StringToText` (`BlueprintMapLibrary.Map_Find` AMRDataJsonMap "locationY")) (`KismetTextLibrary.Conv_StringToText` (`BlueprintMapLibrary.Map_Find` AMRDataJsonMap "locationZ")) (`KismetTextLibrary.Conv_StringToText` (`BlueprintMapLibrary.Map_Find` AMRDataJsonMap "height")) (`KismetTextLibrary.Conv_StringToText` (`BlueprintMapLibrary.Map_Find` AMRDataJsonMap "direction")) (`KismetTextLibrary.Conv_StringToText` (`BlueprintMapLibrary.Map_Find` AMRDataJsonMap "velocity")) (`KismetTextLibrary.Conv_StringToText` (`BlueprintMapLibrary.Map_Find` AMRDataJsonMap "battery")) (`KismetTextLibrary.Conv_StringToText` (`BlueprintMapLibrary.Map_Find` AMRDataJsonMap "collisionEtected"))))

(fn `MakeAMRDataMap_String`
  (params (InAmrType :type String) (InState :type String) (InDestination :type String) (InPositionX :type String) (InPositionY :type String) (InPositionZ :type String) (InHeight :type String) (InDirection :type String) (InVelocity :type String) (InBattery :type String) (InCollisionDetected :type String))
  (returns (AMRAttributes :type "Map of String to String"))
  (return (`|MakeMap` "amrType" InAmrType "locationX" InPositionX "locationY" InPositionY "locationZ" InPositionZ "height" InHeight "direction" InDirection "velocity" InVelocity "state" InState "destination" InDestination "battery" InBattery "collisionEtected" InCollisionDetected)))