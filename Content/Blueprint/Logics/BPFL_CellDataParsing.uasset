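; Blueprint function library that converts factory cell and production-total data to and from key-value maps.
; Two find functions unpack maps by fixed keys: one for cell, process and product fields, the other for daily and monthly results, plans and defect counts.
; The make function builds a post map with the cell keys, but sets only the first four values, from inputs whose names do not match those keys.
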(fn `FindCellDataFromMap`
  (params (InMap :type "Map of String to String (by ref)"))
  (returns (CellID :type String) (CellType :type String) (StartTime :type String) (ProcessTime :type String) (ProcessStatus :type String) (CompletionRate :type String) (ProcessRate :type String) (ProductID :type String) (ProductModel :type String) (ProductColor :type String) (ProductProcessRate :type String) (CustomerID :type String))
  (return (`BlueprintMapLibrary.Map_Find` InMap "cellId") (`BlueprintMapLibrary.Map_Find` InMap "cellType") (`BlueprintMapLibrary.Map_Find` InMap "startTime") (`BlueprintMapLibrary.Map_Find` InMap "processTime") (`BlueprintMapLibrary.Map_Find` InMap "processStatus") (`BlueprintMapLibrary.Map_Find` InMap "completionRate") (`BlueprintMapLibrary.Map_Find` InMap "processRate") (`BlueprintMapLibrary.Map_Find` InMap "productId") (`BlueprintMapLibrary.Map_Find` InMap "productModel") (`BlueprintMapLibrary.Map_Find` InMap "productColor") (`BlueprintMapLibrary.Map_Find` InMap "productProcessRate") (`BlueprintMapLibrary.Map_Find` InMap "customerId")))

(fn `FindTotalDataFromMap`
  (params (InMap :type "Map of String to String (by ref)"))
  (returns (factoryId :type String) (dailyResult :type String) (dailyPlan :type String) (monthlyResult :type String) (monthlyPlan :type String) (defectiveQualityCount :type String) (date :type String))
  (return (`BlueprintMapLibrary.Map_Find` InMap "factoryId") (`BlueprintMapLibrary.Map_Find` InMap "dailyResult") (`BlueprintMapLibrary.Map_Find` InMap "dailyPlan") (`BlueprintMapLibrary.Map_Find` InMap "monthlyResult") (`BlueprintMapLibrary.Map_Find` InMap "monthlyPlan") (`BlueprintMapLibrary.Map_Find` InMap "defectiveQualityCount") (`BlueprintMapLibrary.Map_Find` InMap "date")))

(fn `Make Post Cell Data Map String`
  (params (InRecentStartTime :type String) (InProcessID :type String) (InPorcessStatus :type String) (InCompletionRate :type String))
  (returns (PostCellDataMap :type "Map of String to String"))
  (return (`|MakeMap` "cellId" InRecentStartTime "cellType" InProcessID "startTime" InPorcessStatus "processTime" InCompletionRate "processStatus" "" "completionRate" "" "processRate" "" "productId" "" "productModel" "" "productColor" "" "productProcessRate" "" "customerId")))