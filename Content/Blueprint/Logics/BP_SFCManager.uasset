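; Central manager for a factory scene of AMRs, cells and facilities that starts the simulation and handles camera views.
; On BeginPlay it initializes AMRs, indexes placers by tag, and passes collected data containers to a new widget manager.
; After binding UI and AMR delegates, it connects each AMR's socket and activates it.
; Camera functions target AMRs, floors or the default pawn, with a timeline sliding a clipping box for second-floor viewing.
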(event `self.ReceiveBeginPlay`
  ;[0.1823 0.1823 0.1823] Initialize Game Routine
  (bind _aspawn_sf (cast `/SmartFactory/Blueprint/Logics/Pawn_SF` (`GameplayStatics.GetPlayerPawn` 0)))
  (set `self.DefaultPawnRef` _aspawn_sf)
  (`|ExecutionSequence`
    (:`then_0`
      (for _array_element (`self.AMRRefArray`)
        (`/SmartFactory/Blueprint/AMR/BP/BP_AINavAgent.Initialize AMR DataManagers` _array_element)
        (`self.InitializeWaitingStack`)))
    (:`then_1`
      (`self.Init Widget Manager Routine`))
    (:`then_2`
      ;;[1 1 1] Ready to Start
      (`SFCWidgetManager.ShowWidget` (`self.WidgetManagerRef`) "Main")
      (`KismetSystemLibrary.Delay` 0.4)
      (`self.GameStart`))))

(event `Init Widget Manager Routine`
  (bind _widgetmanagerref (`self.WidgetManagerRef`))
  ;[0.1448 0.1448 0.1448] Initialize Widget Manager Routine
  (bind _returnvalue (`SFCWidgetManager.CreateWidgetManagerInstance` self "/SmartFactory/Widget/BP_SFCWidgetManager.BP_SFCWidgetManager_C"))
  (bind _asbp_sfcwidget_manager (cast `/SmartFactory/Widget/BP_SFCWidgetManager` _returnvalue))
  (`/Engine/EditorBlueprintResources/StandardMacros.IsValid` _asbp_sfcwidget_manager
    (:`Is Valid`
      (set `self.WidgetManagerRef` _asbp_sfcwidget_manager)
      (`SFCWidgetManager.SetPlayerControllerRef` _widgetmanagerref (`GameplayStatics.GetPlayerController` 0))
      (bind _outdatacontainerrefarray (`self.SetAllDataContainerRefs`))
      (bind _output_get (set `self.AllDataContainerRefArray` _outdatacontainerrefarray))
      (`/SmartFactory/Widget/BP_SFCWidgetManager.InitializeWidgetManagerRoutine` _widgetmanagerref self _output_get)
      (`self.CE_BindWidgetFunctions`))))

(event `CE_BindWidgetFunctions`
  ;[0.1531 0.1531 0.1531] ManagerBidnings
  (add `/SmartFactory/Widget/Template/W_MyDropDown.Call OnSelectionChanged` (`/SmartFactory/Widget/MemberWidgets/WBP_AMRManage.W_AMRListDropDown` (`/SmartFactory/Widget/BP_SFCWidgetManager.WBP_AMRManageRef` (`self.WidgetManagerRef`))) (`|CreateDelegate` :!event `SetCameraAMRPawn`))
  (add `/SmartFactory/Widget/MemberWidgets/WBP_SFCMain.ED_WidgetCamOut` (`/SmartFactory/Widget/BP_SFCWidgetManager.WBP_MainRef` (`self.WidgetManagerRef`)) (`|CreateDelegate` :!event `SetCameraDefault`))
  (add `/SmartFactory/Widget/MemberWidgets/WBP_SFCMain.ED_WidgetSecondFloorClicked` (`/SmartFactory/Widget/BP_SFCWidgetManager.WBP_MainRef` (`self.WidgetManagerRef`)) (`|CreateDelegate` :!event `SetCameraFirstFloor`))
  (add `/SmartFactory/Widget/MemberWidgets/WBP_SFCMain.ED_WidgetFirstFloorClicked` (`/SmartFactory/Widget/BP_SFCWidgetManager.WBP_MainRef` (`self.WidgetManagerRef`)) (`|CreateDelegate` :!event `SetCameraSecondFloor`))
  ;[0.1281 0.1281 0.1281] BindAMRDelegates
  (for _array_element (`self.AMRRefArray`)
    (add `/SmartFactory/Blueprint/AMR/BP/BP_AINavAgent.ED_AMRStartWaiting` _array_element (`|CreateDelegate` :!event `OnAMRWaiting`))
    (add `/SmartFactory/Blueprint/AMR/BP/BP_AINavAgent.ED_AMRStartMoving` _array_element (`|CreateDelegate` :!event `CallAMRMoving`))
    (add `/SmartFactory/Blueprint/AMR/BP/BP_AINavAgent.ED_AMRArrivied` _array_element (`|CreateDelegate` :!event `ONAMRMovingArrived`))
    (add `/SmartFactory/Blueprint/AMR/BP/BP_AINavAgent.ED_AMRWorkingDone` _array_element (`|CreateDelegate` :!event `OnAMRWorkingDone`))))

(event `GameStart`
  ;[0.08229 0.08229 0.08229] Game Start
  (for _array_element (`self.AMRRefArray`)
    (`/SmartFactory/Blueprint/AMR/BP/BP_AINavAgent.ConnectSocket` _array_element)
    (`self.ActivateAMR` _array_element)))

(event `/SmartFactory/Blueprint/AMR/BP/BPIF_AMR.ActivateAMR`
  (params (AMRRef :type "/SmartFactory/Blueprint/AMR/BP/BP_AINavAgent Object Reference"))
  (`/SmartFactory/Blueprint/AMR/BP/BP_AINavAgent.SetAMRState` AMRRef "NewEnumerator2"))

(event `/SmartFactory/Blueprint/AMR/BP/BPIF_AMR.ONAMRMovingArrived`
  (params (AMRPlacerRef :type "/SmartFactory/Blueprint/BP_AMRPlacer Object Reference"))
  ;[1 1 1] ONAMR Moving Arrived
)

(event `SetDownClippingBox`
  (bind _clippingboxref (`self.ClippingBoxRef`))
  (bind (_returnvalue_x _returnvalue_y) (`KismetMathLibrary.BreakVector` (`self.K2_GetActorLocation` _clippingboxref)))
  (if (not (`self.bClippingBoxDown`))
    (set `self.bClippingBoxDown` true)
    (bind (_direction `_새_트랙_1`) (`Timeline|타임라인` :!via `PlayFromStart` :!label _label)
      (:`Update`
        (`self.K2_SetActorLocation` _clippingboxref (`KismetMathLibrary.MakeVector` _returnvalue_x _returnvalue_y (`KismetMathLibrary.Lerp` 4000.0 3200.0 `_새_트랙_1`)) false false)))))

(event `SetupClippingBox`
  (if (`self.bClippingBoxDown`)
    (set `self.bClippingBoxDown` false)
    (goto _label :!via `ReverseFromEnd`)))

(fn `InitializeSFCManagerRefernecesRoutine`
  (params (InAMRRefArray :type "Array of /SmartFactory/Blueprint/AMR/BP/BP_AINavAgent Object Reference (by ref)") (InAMRPlacerRefArray :type "Array of /SmartFactory/Blueprint/BP_AMRPlacer Object Reference (by ref)") (InCellRefArray :type "Array of /SmartFactory/Blueprint/BP_Cell Object Reference (by ref)") (InFacilityRefArray :type "Array of /SmartFactory/Blueprint/BP_Facility Object Reference (by ref)"))
  (`self.SetAINavAgentRefs` InAMRRefArray)
  (`self.SetAMRPlacerRefs` InAMRPlacerRefArray)
  (`self.SetCellRefs` InCellRefArray)
  (`self.SetFacilityRefs` InFacilityRefArray))

(fn `InitializeWaitingStack`
  (locals (TempArray :type "Array of Integer"))
  (for (_array_element _array_index) (`self.AMRPlacerRefArray`)
    (bind _output (`|GetArrayItem` (`Actor.Tags` _array_element)))
    (switch `name` _output
      (:`Welding`
        (`KismetArrayLibrary.Array_Add` (`self.WeldingIndexes`) _array_index))
      (:`Painting`
        (`KismetArrayLibrary.Array_Add` (`self.PaintingIndexes`) _array_index))
      (:`Storaging`
        (`BlueprintMapLibrary.Map_Add` (`self.RestFacilities`) _output _array_index :!label _label))
      (:`Charging`
        (goto _label)))))

(fn `Set3DWidgetRefs`
  (params (`3DWidgetTotal` :type "/SmartFactory/Widget/khy/BP_3DWidgetTotal Object Reference"))
  (set `self.3DWidget Total` `3DWidgetTotal`))

(fn `SetAINavAgentRefs`
  (params (`In AMR Ref` :type "Array of /SmartFactory/Blueprint/AMR/BP/BP_AINavAgent Object Reference (by ref)"))
  (set `self.AMRRefArray` `In AMR Ref`))

(fn `SetAllDataContainerRefs`
  (returns (OutDataContainerRefArray :type "Array of SFCDataContainer Object Reference"))
  (locals (DataContainerRefArray :type "Array of SFCDataContainer Object Reference"))
  (bind _total3dwidgetref (`self.Total3DWidgetRef`))
  (`|ExecutionSequence`
    (:`then_0`
      (for _array_element (`self.AMRRefArray`)
        (`/Engine/EditorBlueprintResources/StandardMacros.IsValid` _array_element
          (:`Is Valid`
            (`KismetArrayLibrary.Array_Add` (`local.DataContainerRefArray`) (`/SmartFactory/Blueprint/AMR/BP/BP_AINavAgent.AMRDataContainerRef` _array_element))))))
    (:`then_1`
      (for _array_element_2 (`self.CellRefArray`)
        (`/Engine/EditorBlueprintResources/StandardMacros.IsValid` _array_element_2
          (:`Is Valid`
            (`KismetArrayLibrary.Array_Add` (`local.DataContainerRefArray`) (`/SmartFactory/Blueprint/BP_Cell.DataContainerRef` _array_element_2))))))
    (:`then_2`
      (for _array_element_3 (`self.FacilityRefArray`)
        (`/Engine/EditorBlueprintResources/StandardMacros.IsValid` _array_element_3
          (:`Is Valid`
            (`KismetArrayLibrary.Array_Add` (`local.DataContainerRefArray`) (`/SmartFactory/Blueprint/BP_Facility.DataContainerRef` _array_element_3))))))
    (:`then_3`
      (`/Engine/EditorBlueprintResources/StandardMacros.IsValid` _total3dwidgetref
        (:`Is Valid`
          (`KismetArrayLibrary.Array_Add` (`local.DataContainerRefArray`) (`/SmartFactory/Widget/khy/BP_3DWidgetTotal.DataContainer` _total3dwidgetref))
          (return (`local.DataContainerRefArray`)))))))

(fn `SetAllDataContainersFromActors`
  (params (AllDataContainerRefArray :type "Array of SFCDataContainer Object Reference"))
  (set `self.AllDataContainerRefArray` AllDataContainerRefArray))

(fn `SetAMRPlacerRefs`
  (params (AMRPlacerRefs :type "Array of /SmartFactory/Blueprint/BP_AMRPlacer Object Reference"))
  (set `self.AMRPlacerRefArray` AMRPlacerRefs))

(fn `SetCameraAMRPawn`
  (params (SelectionAMR :type String) (SeletionType :type "ESelectInfo Enum" :default "OnKeyPress"))
  (`PlayerController.SetViewTargetWithBlend` (`GameplayStatics.GetPlayerController` 0) (`|GetArrayItem` (`self.AMRRefArray`) (`KismetArrayLibrary.Array_Find` (`/SmartFactory/Widget/MemberWidgets/WBP_AMRManage.AMRActorNames` (`/SmartFactory/Widget/BP_SFCWidgetManager.WBP_AMRManageRef` (`self.WidgetManagerRef`))) SelectionAMR)) 0.1 "VTBlend_Linear" 0.0 false))

(fn `SetCameraDefault`
  (bind _defaultpawnref (`self.DefaultPawnRef`))
  (`PlayerController.SetViewTargetWithBlend` (`GameplayStatics.GetPlayerController` 0) _defaultpawnref 0.1 "VTBlend_Linear" 0.0 false)
  (`self.SetupClippingBox`)
  (`self.K2_SetActorLocation` _defaultpawnref (1500.0 1700.0 1500.0) false false))

(fn `SetCameraFirstFloor`
  (`self.K2_SetActorTransform` (`GameplayStatics.GetPlayerPawn` 0) (`KismetMathLibrary.MakeTransform` (2359.609742 1063.26225 662.594765) (`KismetMathLibrary.MakeRotator` 0.0 -21.200001 97.333506)) false false))

(fn `SetCameraSecondFloor`
  (`PlayerController.SetViewTargetWithBlend` (`GameplayStatics.GetPlayerController` 0) (`self.SecondFloorCam`) 0.1 "VTBlend_Linear" 0.0 false)
  (`self.SetDownClippingBox`))

(fn `SetCellRefs`
  (params (InCellRefArray :type "Array of /SmartFactory/Blueprint/BP_Cell Object Reference"))
  (set `self.CellRefArray` InCellRefArray))

(fn `SetFacilityRefs`
  (params (FacilityRefArray :type "Array of /SmartFactory/Blueprint/BP_Facility Object Reference"))
  (set `self.FacilityRefArray` FacilityRefArray))

(fn `SetRestActorRefs`
  (params (SecondFloorCam :type "CameraActor Object Reference") (ClippingBoxRef :type "/SmartFactory/Blueprint/Environment/BP_ClippingBox Object Reference") (Total3DWidgetRef :type "/SmartFactory/Widget/khy/BP_3DWidgetTotal Object Reference"))
  (set `self.SecondFloorCam` SecondFloorCam)
  (set `self.ClippingBoxRef` ClippingBoxRef)
  (set `self.Total3DWidgetRef` Total3DWidgetRef))

(fn `UserConstructionScript`)