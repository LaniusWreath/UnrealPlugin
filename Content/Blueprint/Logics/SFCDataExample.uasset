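; Example Blueprint showcasing the SFC data plugin's API for collecting and managing data, with every node chain left unconnected to any event.
; The collecting samples create WebSocket and HTTP managers, then show connection, messaging, GET requests and delegate binding to empty handler events.
; The managing samples build generic and JSON data structs, parse JSON strings, save text to file and create or update data container objects.
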(event `OnMessageReceivedEvent_이벤트`
  (params (ReceivedMessage :type String))
  ;[0.4202 0.4719 1 1 37] Collecting
  ;;[0 0 0] WebSocket
)

(event `OnDynamicRequestingEvent_이벤트`
  ;[0.4202 0.4719 1 1 37] Collecting
  ;;[0 0 0] HTTP
)