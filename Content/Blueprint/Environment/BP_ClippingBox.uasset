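; BP_ClippingBox is an environment actor that publishes an oriented box, defined by its Cube component, for materials to use, presumably for clipping.
; It writes the Cube's world location, scale and three axis vectors into the MPC_ClippingParameters material parameter collection.
; The construction script sets these values at construction, and Tick repeats the same writes through CalculateClipping so the collection follows the box at runtime.
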(event `self.ReceiveTick`
  (params (DeltaSeconds :type "Float (single-precision)"))
  (`self.CalculateClipping`))

(fn `CalculateClipping`
  (bind _cube (`self.Cube`))
  (bind _cube_2 (`self.Cube`))
  (`KismetMaterialLibrary.SetVectorParameterValue` "/SmartFactory/Material/Clipping/MPC_ClippingParameters.MPC_ClippingParameters" "Location" (`KismetMathLibrary.Conv_VectorToLinearColor` (`SceneComponent.K2_GetComponentLocation` _cube)))
  (`KismetMaterialLibrary.SetVectorParameterValue` "/SmartFactory/Material/Clipping/MPC_ClippingParameters.MPC_ClippingParameters" "Bounds" (`KismetMathLibrary.Conv_VectorToLinearColor` (`SceneComponent.K2_GetComponentScale` _cube)))
  (`KismetMaterialLibrary.SetVectorParameterValue` "/SmartFactory/Material/Clipping/MPC_ClippingParameters.MPC_ClippingParameters" "X" (`KismetMathLibrary.Conv_VectorToLinearColor` (`SceneComponent.GetForwardVector` _cube_2)))
  (`KismetMaterialLibrary.SetVectorParameterValue` "/SmartFactory/Material/Clipping/MPC_ClippingParameters.MPC_ClippingParameters" "Y" (`KismetMathLibrary.Conv_VectorToLinearColor` (`SceneComponent.GetRightVector` _cube_2)))
  (`KismetMaterialLibrary.SetVectorParameterValue` "/SmartFactory/Material/Clipping/MPC_ClippingParameters.MPC_ClippingParameters" "Z" (`KismetMathLibrary.Conv_VectorToLinearColor` (`SceneComponent.GetUpVector` _cube_2))))

(fn `UserConstructionScript`
  (bind _cube (`self.Cube`))
  (bind _cube_2 (`self.Cube`))
  (`KismetMaterialLibrary.SetVectorParameterValue` "/SmartFactory/Material/Clipping/MPC_ClippingParameters.MPC_ClippingParameters" "Location" (`KismetMathLibrary.Conv_VectorToLinearColor` (`SceneComponent.K2_GetComponentLocation` _cube)))
  (`KismetMaterialLibrary.SetVectorParameterValue` "/SmartFactory/Material/Clipping/MPC_ClippingParameters.MPC_ClippingParameters" "Bounds" (`KismetMathLibrary.Conv_VectorToLinearColor` (`SceneComponent.K2_GetComponentScale` _cube)))
  (`KismetMaterialLibrary.SetVectorParameterValue` "/SmartFactory/Material/Clipping/MPC_ClippingParameters.MPC_ClippingParameters" "X" (`KismetMathLibrary.Conv_VectorToLinearColor` (`SceneComponent.GetForwardVector` _cube_2)))
  (`KismetMaterialLibrary.SetVectorParameterValue` "/SmartFactory/Material/Clipping/MPC_ClippingParameters.MPC_ClippingParameters" "Y" (`KismetMathLibrary.Conv_VectorToLinearColor` (`SceneComponent.GetRightVector` _cube_2)))
  (`KismetMaterialLibrary.SetVectorParameterValue` "/SmartFactory/Material/Clipping/MPC_ClippingParameters.MPC_ClippingParameters" "Z" (`KismetMathLibrary.Conv_VectorToLinearColor` (`SceneComponent.GetUpVector` _cube_2))))