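; BP_Facility is a production facility actor that stores data received over HTTP.
; On BeginPlay it creates an empty data container and an SFCHttpManager instance, then binds to the manager's dynamic request event.
; OnHTTPResponseReceived parses the JSON response into a map and writes it with the raw string into the container, keyed by display name.
; SetServerURL stores URL and facility ID, while activate, stop and GET-request functions are empty stubs.
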(event `self.ReceiveBeginPlay`
  (`self.InitializeDataManagers`))

(fn `ActivateFacility`)

(fn `InitializeDataManagers`
  (`|ExecutionSequence`
    (:`then_0`
      (bind _returnvalue (`SFCDataManageUtilities.CreateEmptyDataContainer` self))
      (set `self.DataContainerRef` _returnvalue))
    (:`then_1`
      (bind _returnvalue_2 (`SFCHttpManager.CreateHttpManagerInstance` self "/Script/SmartFactory.SFCHttpManager"))
      (set `self.HTTPManagerRef` _returnvalue_2))
    (:`then_2`
      (add `SFCHttpManager.OnDynamicRequestingEvent` (`self.HTTPManagerRef`) (`|CreateDelegate` :!event `OnHTTPResponseReceived`)))))

(fn `MakeGetRequest`)

(fn `OnHTTPResponseReceived`
  (bind _returnvalue (`SFCHttpManager.GetTempResultResponseString` (`self.HTTPManagerRef`)))
  (bind _returnvalue_2 (`SFCDataManageUtilities.ParseJsonStringToMap` _returnvalue))
  (`SFCDataManageUtilities.UpdateDataContainer` (`self.DataContainerRef`) (make `GenericData` (`KismetSystemLibrary.GetDisplayName` self) _returnvalue _returnvalue_2)))

(fn `SetServerURL`
  (params (InUrl :type String) (InFacilityID :type String))
  (set `self.Url` InUrl)
  (set `self.FacilityID` InFacilityID))

(fn `StopFacility`)

(fn `UserConstructionScript`)