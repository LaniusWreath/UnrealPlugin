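; BP_Conveyor is a conveyor Blueprint whose only live behavior is activating its Audio component on BeginPlay.
; HTTP and WebSocket handlers parse received JSON into maps without using the result, and the nodes that create and bind their managers never run.
; The remaining graph holds disconnected sample calls to SFC networking, data-container, string-parsing and file-saving utilities, with empty placeholder inputs.
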(event `self.ReceiveBeginPlay`
  (`ActorComponent.Activate` (`self.Audio`) true))

(event `OnWebsocketMessageReceived`
  (params (ReceivedMessage :type String))
  ;[0.2871 0.327 0.674] WebSocket
  (`SFCDataManageUtilities.ParseJsonStringToMap` ReceivedMessage))

(event `OnHTTPResponseReceived`
  ;[1 0.3677 0.3677] HTTP
  (`SFCDataManageUtilities.ParseJsonStringToMap` (`SFCHttpManager.GetResultResponseString` (`self.HTTPManagerRef`))))

(fn `UserConstructionScript`)