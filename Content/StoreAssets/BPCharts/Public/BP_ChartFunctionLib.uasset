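; Blueprint function library of math helpers for chart widgets, including radar charts.
; Derives an axis upper limit by padding "1" with a zero per digit of the rounded maximum, and normalizes values to fractions of their sum.
; Radar helpers place polygon corners and data points at even angles from the top around the widget center, optionally closing the grid outline.
; Also generates random whole-number test data.
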(fn `GetDataNormalizeValues`
  (params (ValuesArray :type "Array of Float (double-precision)"))
  (returns (NormalizeValues :type "Array of Float (double-precision)"))
  (locals (Sum :type "Float (double-precision)") (Normalize :type "Array of Float (double-precision)"))
  (set `local.Sum` 0.0)
  (`KismetArrayLibrary.Array_Clear` (`local.Normalize`))
  (for _array_element ValuesArray
    (set `local.Sum` (+ (`local.Sum`) _array_element)))
  (for _array_element_2 ValuesArray
    (`KismetArrayLibrary.Array_Add` (`local.Normalize`) (/ _array_element_2 (`local.Sum`))))
  (return (`local.Normalize`)))

(fn `GetDataUpperLimit`
  (params (ValuesArray :type "Array of Float (double-precision)"))
  (returns (TheUpperLimit :type "Float (double-precision)"))
  (locals (LimitString :type String))
  (bind (_indexofmaxvalue _maxvalue) (`KismetMathLibrary.MaxOfFloatArray` ValuesArray))
  (if (> (`KismetArrayLibrary.Array_Length` ValuesArray) 2)
    (if (> _maxvalue 1.0)
      (set `local.LimitString` "1")
      (for _ (range 1 (+ (`KismetStringLibrary.Len` (`KismetStringLibrary.Conv_IntToString` (`KismetMathLibrary.Round` _maxvalue))) 1))
        (set `local.LimitString` (`KismetStringLibrary.Concat_StrStr` (`local.LimitString`) "0")))
      (return (`KismetStringLibrary.Conv_StringToDouble` (`local.LimitString`)))
      (else
        (return 1.0)))
    (else
      (return 0.0))))

(fn `GetRadarDataPoints`
  (params (DataLengthInWidget :type "Array of Float (double-precision)") (`ＷidgetHalfWidth` :type "Float (double-precision)"))
  (returns (DataPoints :type "Array of Vector2D Structure"))
  (locals (Points :type "Array of Vector2D Structure"))
  (bind _points (`local.Points`))
  (`KismetArrayLibrary.Array_Clear` (`local.Points`))
  (for (_array_element _array_index) DataLengthInWidget
    (bind _returnvalue (+ (* (/ 360.0 (`KismetMathLibrary.Conv_IntToDouble` (`KismetArrayLibrary.Array_Length` DataLengthInWidget))) _array_index) -90.0))
    (`KismetArrayLibrary.Array_Add` (`local.Points`) (`KismetMathLibrary.MakeVector2D` (+ (* (`KismetMathLibrary.DegCos` _returnvalue) _array_element) `ＷidgetHalfWidth`) (+ `ＷidgetHalfWidth` (* _array_element (`KismetMathLibrary.DegSin` _returnvalue))))))
  (`KismetArrayLibrary.Array_Add` _points (`|GetArrayItem` _points))
  (return _points))

(fn `GetRadarSidePoints`
  (params (SideNum :type Integer) (RadiusLength :type "Float (double-precision)") (Closed :type Boolean) (WidgetHalfWidth :type "Float (double-precision)"))
  (returns (RadarPoints :type "Array of Vector2D Structure"))
  (locals (Points :type "Array of Vector2D Structure"))
  (bind _points (`local.Points`))
  (`KismetArrayLibrary.Array_Clear` (`local.Points`))
  (for _index (range SideNum)
    (bind _returnvalue (+ (* (/ 360.0 (`KismetMathLibrary.Conv_IntToDouble` SideNum)) _index) -90.0))
    (`KismetArrayLibrary.Array_Add` (`local.Points`) (`KismetMathLibrary.MakeVector2D` (+ (* (`KismetMathLibrary.DegCos` _returnvalue) RadiusLength) WidgetHalfWidth) (+ WidgetHalfWidth (* RadiusLength (`KismetMathLibrary.DegSin` _returnvalue))))))
  (if Closed
    (`KismetArrayLibrary.Array_Add` _points (`|GetArrayItem` _points)))
  (return _points))

(fn `GetRandomData`
  (params (DataNum :type Integer) (Min :type Integer) (Max :type Integer))
  (returns (Return :type "Array of Float (double-precision)"))
  (locals (RandomData :type "Array of Float (double-precision)"))
  (bind _randomdata (`local.RandomData`))
  (`KismetArrayLibrary.Array_Clear` _randomdata)
  (for _ (range DataNum)
    (`KismetArrayLibrary.Array_Add` _randomdata (`KismetMathLibrary.Conv_IntToDouble` (`KismetMathLibrary.RandomIntegerInRange` Min Max))))
  (return (`local.RandomData`)))