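; BP_BoxQueue is a waiting point that hands arriving BP_SpawnedObject boxes to a rack loader in arrival order.
; Box overlaps store each object in a map keyed by game time, whose sorted keys identify the oldest.
; Each overlap or loader movement-end event halts that oldest box, then loads and dequeues it if the loader is idle.
; The construction script places the Scene component at TargetLocation.
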(event `self.ReceiveBeginPlay`
  (bind _rackloaderref (`self.RackLoaderRef`))
  ;[1 1 1] Upon the loader finishing its work
  (`/Engine/EditorBlueprintResources/StandardMacros.IsValid` _rackloaderref
    (:`Is Valid`
      (add `/SmartFactory/BP_RackLoader.OnMovementEnd` _rackloaderref (delegate `LoadOnMovementEnd`)))))

(event `LoadOnMovementEnd`
  ;[1 1 1] Upon the loader finishing its work
  (`self.BoxToLoader`))

(event `self.Box.OnComponentBeginOverlap`
  (params (OverlappedComponent :type "PrimitiveComponent Object Reference") (OtherActor :type "Actor Object Reference") (OtherComp :type "PrimitiveComponent Object Reference") (OtherBodyIndex :type Integer) (bFromSweep :type Boolean) (SweepResult :type "HitResult Structure (by ref)"))
  (cast `/SmartFactory/BP_SpawnedObject` OtherActor)
  (`BlueprintMapLibrary.Map_Add` (`self.OverlappedActorsMap`) (`KismetSystemLibrary.GetGameTimeInSeconds`) OtherActor)
  (`self.BoxToLoader`))

(fn `BoxToLoader`
  (bind _rackloaderref (`self.RackLoaderRef`))
  (bind (_key _value) (`self.GetFirstOverlappingBox`))
  (bind _asbp_spawned_object (cast `/SmartFactory/BP_SpawnedObject` _value))
  ;[1 1 1] Queue에 담기면 멈춰!
  (set `/SmartFactory/BP_SpawnedObject.bMoving` false _asbp_spawned_object)
  ;[1 1 1] Queue에 Box 담아뒀다가 Loader가 동작하고 있지 않을 때, Loader에 올리기
  (if (not (`/SmartFactory/BP_RackLoader.bMoving` _rackloaderref))
    (`/SmartFactory/BP_RackLoader.OnLoad` _rackloaderref _asbp_spawned_object)
    (`BlueprintMapLibrary.Map_Remove` (`self.OverlappedActorsMap`) _key)))

(fn `GetFirstOverlappingBox`
  (returns (Key :type "Float (double-precision)") (Value :type "Actor Object Reference"))
  (locals (TimeArray :type "Array of Float (double-precision)"))
  (bind _overlappedactorsmap (`self.OverlappedActorsMap`))
  (bind _output (`|GetArrayItem` (`local.TimeArray`)))
  (bind (_value _returnvalue) (`BlueprintMapLibrary.Map_Find` (`self.OverlappedActorsMap`) _output))
  (if (not (`BlueprintMapLibrary.Map_IsEmpty` _overlappedactorsmap))
    (bind _keys (`BlueprintMapLibrary.Map_Keys` _overlappedactorsmap))
    (bind _output_get (set `local.TimeArray` _keys))
    (`KismetArrayLibrary.SortFloatArray` _output_get)
    (if _returnvalue
      (return _output _value))))

(fn `UserConstructionScript`
  (`SceneComponent.K2_SetRelativeLocation` (`self.Scene`) (`self.TargetLocation`) false false))